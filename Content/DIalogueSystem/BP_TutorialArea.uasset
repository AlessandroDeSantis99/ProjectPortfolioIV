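; BP_TutorialArea is a one-shot trigger that starts dialogue when a BP_CharacterBuild overlaps its Cube.
; It caches the level's BP_DialogueManager on BeginPlay and plays a 2D sound on overlap.
; IsBelicaDialogue selects the tutorial or collectible channel, whose start flag, content and display duration it writes directly into the manager.
; The actor then destroys itself.
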(event OnComponentBeginOverlap(Cube)
  (params (OverlappedComponent :type Primitive%20Component%20Object%20Reference) (OtherActor :type Actor%20Object%20Reference) (OtherComp :type Primitive%20Component%20Object%20Reference) (OtherBodyIndex :type Integer) (bFromSweep :type Boolean) (SweepResult :type Hit%20Result%20Structure%20%28by%20ref%29))
  (bind _dialoguemanager (Variables|Default|GetDialogueManager))
  (Utilities|Casting|CastToBP_CharacterBuild OtherActor)
  (Audio|PlaySound2D (Variables|Default|GetSound) 1.0 1.0 0.0 0 0)
  (if (Variables|Default|GetIsBelicaDialogue?)
    (Variables|/Game/DIalogueSystem/BP_DialogueManager.BP_DialogueManager_C|SetStartDialogueTutorial? _dialoguemanager true)
    (Variables|/Game/DIalogueSystem/BP_DialogueManager.BP_DialogueManager_C|SetDialogueTutorial _dialoguemanager (Variables|Default|GetDialogueToDisplayOnTutorial))
    (Variables|/Game/DIalogueSystem/BP_DialogueManager.BP_DialogueManager_C|SetSetTimeToDestryDial_Tutorial _dialoguemanager (Variables|Default|GetDialogueTutorialDuration))
    (else
      (Variables|/Game/DIalogueSystem/BP_DialogueManager.BP_DialogueManager_C|SetStartDialogue? _dialoguemanager true)
      (Variables|/Game/DIalogueSystem/BP_DialogueManager.BP_DialogueManager_C|SetCollectbaleTaken _dialoguemanager (Variables|Default|GetDialogueToDisplayOnCollectible))
      (Variables|/Game/DIalogueSystem/BP_DialogueManager.BP_DialogueManager_C|SetSetTimeToDestryDial_collectible _dialoguemanager (Variables|Default|GetDialogueCollectibleDuration))))
  (Actor|DestroyActor))

(event EventBeginPlay
  (bind _returnvalue (Actor|GetActorOfClass "/Game/DIalogueSystem/BP_DialogueManager.BP_DialogueManager_C"))
  (Variables|Default|SetDialogueManager _returnvalue))

(fn ConstructionScript)