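; BP_DialogueManager shows timed dialogue widgets, starting with the first dialogue at level start.
; Tick polls the StartDialogue flag, which BeginPlay sets, and a DoOnce gate prevents repeat triggers while a dialogue is showing.
; The collectible count picks the dialogue from an array and WD_Dialogue is added to the viewport.
; After a delay read from a durations array, it removes the widget, clears the flag and resets the gate.
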(event EventBeginPlay
  ;[0.4175 0.3065 1] Primo dialogo inizio livello
  (Variables|Default|SetStartDialogue? true)
  (Variables|Default|SetDialogueToPlay (Utilities|Array|Get(acopy) (Variables|Default|GetDialogues) (Variables|Default|GetCollectbaleTaken))))

(event EventTick
  (params (DeltaSeconds :type Float%20%28single-precision%29))
  (if (Variables|Default|GetStartDialogue?)
    (Utilities|FlowControl|DoOnce false :!label _label
      (:Completed
        (Variables|Default|SetDialogueToPlay (Utilities|Array|Get(acopy) (Variables|Default|GetDialogues) (Variables|Default|GetCollectbaleTaken)))
        (bind _returnvalue (UserInterface|CreateWidget "/Game/DIalogueSystem/WD_Dialogue.WD_Dialogue_C"))
        (UserInterface|Viewport|AddtoViewport _returnvalue 0)
        (Utilities|FlowControl|Delay (Utilities|Array|Get(acopy) (Variables|Default|GetTimeToDestroyDialogues) (Variables|Default|GetSetTimeToDestryDial)))
        (Widget|RemovefromParent _returnvalue)
        (Variables|Default|SetStartDialogue? false)
        (goto _label Reset)))))

(fn ConstructionScript)