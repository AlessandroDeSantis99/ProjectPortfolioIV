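; BP_ProjectileAI is a homing projectile actor that chases the player and destroys itself on contact.
; It caches the player reference on BeginPlay, then each Tick AimToPlayer offsets it toward the player's current location at Speed, scaled by delta time, without sweep or rotation.
; A Sphere overlap with Bp_CharacterController destroys the projectile; no damage is applied here.
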(event OnComponentBeginOverlap(Sphere)
  (params (OverlappedComponent :type Primitive%20Component%20Object%20Reference) (OtherActor :type Actor%20Object%20Reference) (OtherComp :type Primitive%20Component%20Object%20Reference) (OtherBodyIndex :type Integer) (bFromSweep :type Boolean) (SweepResult :type Hit%20Result%20Structure%20%28by%20ref%29))
  ;[1 1 1] Destroy himself when player hit
  (Utilities|Casting|CastToBp_CharacterController OtherActor)
  (Actor|DestroyActor))

(event EventBeginPlay
  (bind _playeristance (CallFunction|GetPlayerIstance))
  (Variables|Default|SetPlayer _playeristance))

(event EventTick
  (params (DeltaSeconds :type Float%20%28single-precision%29))
  (CallFunction|AimtoPlayer (Variables|Default|GetSpeed) DeltaSeconds))

(fn ConstructionScript)

(fn AimtoPlayer
  (params (Speed :type Float%20%28single-precision%29) (DeltaTime :type Float%20%28single-precision%29))
  (Transformation|AddActorWorldOffset (* (* (Math|Vector|Normalize (- (Transformation|GetActorLocation (Variables|Default|GetPlayer)) (Transformation|GetActorLocation))) Speed) DeltaTime)))