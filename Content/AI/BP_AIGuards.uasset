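; AI guard Blueprint that spots the player and shows a one-time alert.
; PawnSensing marks the player visible, and the first sighting reveals a TextRender exclamation mark and immediately stops the guard's movement.
; Tick clears the visible flag once the player leaves the set range, but never resets the first-sighting alert.
; PlayerSeen and QTE functions are unfinished stubs that never run.
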(event OnSeePawn(PawnSensing)
  (params (Pawn :type Pawn%20Object%20Reference))
  ;[0.5441 0.4626 1] Has seen player
  (Variables|Default|SetIsPlayerVisible? true)
  ;[1 0.4987 0.5326] Exclamation mark
  (if (Variables|Default|GetIsPlayerSeenFirstTime?)
    (Variables|Default|SetIsPlayerSeenFirstTime? false)
    (Rendering|SetVisibility (Variables|Default|GetTextRender) true false)
    ;[0.551 1 0.5322] Allert stop
    (Components|Movement|StopMovementImmediately (Variables|Character|GetCharacterMovement))))

(event EventTick
  (params (DeltaSeconds :type Float%20%28single-precision%29))
  (if (Variables|Default|GetIsPlayerVisible?)
    (bind _isinrange_ (CallFunction|IsPlayerinPawnRange? (Variables|Default|GetPlayer) self (Variables|Default|GetIn%20Range%20Distance)))
    (if (not _isinrange_)
      (Variables|Default|SetIsPlayerVisible? false))))

(event EventBeginPlay
  (bind _playeristance (CallFunction|GetPlayerIstance))
  (Variables|Default|SetPlayer _playeristance))

(fn ConstructionScript)