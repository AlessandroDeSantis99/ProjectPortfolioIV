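; BP_WallAlternate is a stealth wall with two trigger colliders that hide a crouching player from enemies.
; BeginPlay caches all Bp_enemyBuild actors and positions both colliders from variables.
; Each tick, a crouched player overlapping either collider clears IsPlayerVisible on enemies not flagged immune.
; An enemy entering a collider disables it and enables the other, after a short delay from Collider2, so the hiding zone alternates.
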(event OnComponentBeginOverlap(Collider2)
  (params (OverlappedComponent :type Primitive%20Component%20Object%20Reference) (OtherActor :type Actor%20Object%20Reference) (OtherComp :type Primitive%20Component%20Object%20Reference) (OtherBodyIndex :type Integer) (bFromSweep :type Boolean) (SweepResult :type Hit%20Result%20Structure%20%28by%20ref%29))
  (Utilities|Casting|CastToBp_enemyBuild OtherActor)
  (Collision|SetCollisionEnabled (Variables|Default|GetCollider2) "NoCollision")
  (Utilities|FlowControl|Delay 0.2)
  (Collision|SetCollisionEnabled (Variables|Default|GetCollider1) "QueryAndPhysics"))

(event OnComponentBeginOverlap(Collider1)
  (params (OverlappedComponent :type Primitive%20Component%20Object%20Reference) (OtherActor :type Actor%20Object%20Reference) (OtherComp :type Primitive%20Component%20Object%20Reference) (OtherBodyIndex :type Integer) (bFromSweep :type Boolean) (SweepResult :type Hit%20Result%20Structure%20%28by%20ref%29))
  (Utilities|Casting|CastToBp_enemyBuild OtherActor)
  (Collision|SetCollisionEnabled (Variables|Default|GetCollider1) "NoCollision")
  (Collision|SetCollisionEnabled (Variables|Default|GetCollider2) "QueryAndPhysics"))

(event EventBeginPlay
  (bind _collider1 (Variables|Default|GetCollider1))
  (bind _collider2 (Variables|Default|GetCollider2))
  (bind _scale_collider_1 (Variables|Default|GetScale%20collider%201))
  (bind _scale_collider_2 (Variables|Default|GetScale%20collider%202))
  (bind _outactors (Actor|GetAllActorsOfClass "/Game/Character/Character_Build/Guards/Bp_enemyBuild.Bp_enemyBuild_C"))
  (Variables|Default|SetEnemies _outactors)
  (Transformation|SetWorldLocation _collider1 (Variables|Default|GetLocation%20Collider1) false true)
  (Transformation|SetWorldLocation _collider2 (Variables|Default|GetLocation%20Collider2) false true)
  (Transformation|SetWorldScale3D _collider2 (Math|Vector|MakeVector (.x _scale_collider_2) (.y _scale_collider_2) (.z _scale_collider_2)))
  (Transformation|SetWorldScale3D _collider1 (Math|Vector|MakeVector (.x _scale_collider_1) (.y _scale_collider_1) (.z _scale_collider_1)))
  (Transformation|SetWorldRotation _collider1 (Math|Conversions|RotationFromXVector (Variables|Default|GetRotationCollider1)) false false)
  (Transformation|SetWorldRotation _collider2 (Math|Conversions|RotationFromXVector (Variables|Default|GetRotationCollider2)) false false))

(event EventTick
  (params (DeltaSeconds :type Float%20%28single-precision%29))
  (if (Collision|IsOverlappingActor (Variables|Default|GetCollider2) (Game|Player|GetPlayerPawn 0) :!class /Script/Engine.PrimitiveComponent)
    (bind _asbp_character_build (Utilities|Casting|CastToBP_CharacterBuild (Game|Player|GetPlayerPawn 0)))
    (if (Variables|/Game/Character/Character_Build/BP_CharacterBuild.BP_CharacterBuild_C|GetIsCrouching? _asbp_character_build)
      (for _array_element (Variables|Default|GetEnemies)
        (if (not (Variables|/Game/Character/Character_Build/Guards/Bp_enemyBuild.Bp_enemyBuild_C|GetIsImmuneToWallAlternate _array_element))
          (Variables|/Game/Character/Character_Build/Guards/Bp_enemyBuild.Bp_enemyBuild_C|SetIsPlayerVisible? _array_element false)
          (if (Collision|IsOverlappingActor (Variables|Default|GetCollider1) (Game|Player|GetPlayerPawn 0) :!class /Script/Engine.PrimitiveComponent)
            (bind _asbp_character_build_2 (Utilities|Casting|CastToBP_CharacterBuild (Game|Player|GetPlayerPawn 0)))
            (if (Variables|/Game/Character/Character_Build/BP_CharacterBuild.BP_CharacterBuild_C|GetIsCrouching? _asbp_character_build_2)
              (for _array_element_2 (Variables|Default|GetEnemies)
                (if (not (Variables|/Game/Character/Character_Build/Guards/Bp_enemyBuild.Bp_enemyBuild_C|GetIsImmuneToWallAlternate _array_element_2))
                  (Variables|/Game/Character/Character_Build/Guards/Bp_enemyBuild.Bp_enemyBuild_C|SetIsPlayerVisible? _array_element_2 false))))))))
    (else
      (if (Collision|IsOverlappingActor (Variables|Default|GetCollider1) (Game|Player|GetPlayerPawn 0) :!class /Script/Engine.PrimitiveComponent)
        (bind _asbp_character_build_3 (Utilities|Casting|CastToBP_CharacterBuild (Game|Player|GetPlayerPawn 0)))
        (if (Variables|/Game/Character/Character_Build/BP_CharacterBuild.BP_CharacterBuild_C|GetIsCrouching? _asbp_character_build_3)
          (for _array_element_3 (Variables|Default|GetEnemies)
            (if (not (Variables|/Game/Character/Character_Build/Guards/Bp_enemyBuild.Bp_enemyBuild_C|GetIsImmuneToWallAlternate _array_element_3))
              (Variables|/Game/Character/Character_Build/Guards/Bp_enemyBuild.Bp_enemyBuild_C|SetIsPlayerVisible? _array_element_3 false))))))))

(fn ConstructionScript)