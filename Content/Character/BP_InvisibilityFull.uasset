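; BP_InvisibilityFull is an invisibility zone that hides the player from enemies while the player overlaps its Cube.
; On BeginPlay it caches every Bp_enemyBuild actor in an Enemies array.
; Each Tick it polls the overlap, confirms the player pawn is a BP_CharacterBuild, and sets IsPlayerVisible to false on every cached enemy.
; Nothing here restores visibility when the overlap ends.
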(event EventTick
  (params (DeltaSeconds :type Float%20%28single-precision%29))
  (if (Collision|IsOverlappingActor (Variables|Default|GetCube) (Game|Player|GetPlayerPawn 0) :!class /Script/Engine.PrimitiveComponent)
    (Utilities|Casting|CastToBP_CharacterBuild (Game|Player|GetPlayerPawn 0))
    (for _array_element (Variables|Default|GetEnemies)
      (Variables|/Game/Character/Character_Build/Guards/Bp_enemyBuild.Bp_enemyBuild_C|SetIsPlayerVisible? _array_element false))))

(event EventBeginPlay
  (bind _outactors (Actor|GetAllActorsOfClass "/Game/Character/Character_Build/Guards/Bp_enemyBuild.Bp_enemyBuild_C"))
  (Variables|Default|SetEnemies _outactors))

(fn ConstructionScript)