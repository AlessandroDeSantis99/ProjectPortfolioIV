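; BP_InvisibilityCrouch is an actor that hides a crouching player from enemies while the player overlaps it.
; It caches every Bp_enemyBuild at BeginPlay, then polls overlap and the character's crouch state each Tick.
; While both hold, it clears IsPlayerVisible on each enemy at least 200 units from the player.
; It never sets the flag back to true.
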(event EventTick
  (params (DeltaSeconds :type Float%20%28single-precision%29))
  (bind _returnvalue (Game|Player|GetPlayerPawn 0))
  (if (Collision|IsOverlappingActor _returnvalue :!class /Script/Engine.Actor)
    (bind _asbp_character_build (Utilities|Casting|CastToBP_CharacterBuild (Game|Player|GetPlayerPawn 0)))
    (if (Variables|/Game/Character/Character_Build/BP_CharacterBuild.BP_CharacterBuild_C|GetIsCrouching? _asbp_character_build)
      (for _array_element (Variables|Default|GetEnemies)
        (if (not (< (Math|Vector|VectorLength (- (Transformation|GetActorLocation _returnvalue) (Transformation|GetActorLocation _array_element))) 2e+02))
          (Variables|/Game/Character/Character_Build/Guards/Bp_enemyBuild.Bp_enemyBuild_C|SetIsPlayerVisible? _array_element false))))))

(event EventBeginPlay
  (bind _outactors (Actor|GetAllActorsOfClass "/Game/Character/Character_Build/Guards/Bp_enemyBuild.Bp_enemyBuild_C"))
  (Variables|Default|SetEnemies _outactors))

(fn ConstructionScript)