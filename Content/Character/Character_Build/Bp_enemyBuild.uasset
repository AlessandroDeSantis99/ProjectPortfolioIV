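; Enemy guard character that spots the player and resolves close encounters through a slow-motion quick-time takedown.
; PawnSensing raises an exclamation alert on first sighting, and Tick range checks gate the QTE behind HasAlreadyShoot.
; The QTE unpossesses the AI, applies CustomTimeDilation to guards and player, shows WB_QTE and increments QTEManager's seen count.
; Winning disables this enemy's movement and collision, while a timeout disables the player's and reloads DefaultMap.
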(event OnSeePawn(PawnSensing)
  (params (Pawn :type Pawn%20Object%20Reference))
  ;[0.5441 0.4626 1] Has seen player
  (Variables|Default|SetIsPlayerVisible? true)
  ;[1 0.4987 0.5326] Exclamation mark
  (if (Variables|Default|GetIsPlayerSeenFirstTime?)
    (Variables|Default|SetIsPlayerSeenFirstTime? false)
    (Rendering|SetVisibility (Variables|Default|GetTextRender) true false)
    ;[0.551 1 0.5322] Allert stop
    (Components|Movement|StopMovementImmediately (Variables|Character|GetCharacterMovement))))

(event EventTick
  (params (DeltaSeconds :type Float%20%28single-precision%29))
  (bind _self self)
  (bind _qtemanager (Variables|Default|GetQTEManager))
  (bind _returnvalue (AI|GetAIController _self))
  (if (Variables|Default|GetIsStartingQTE)
    ;[1 0.1661 0.9631] QTE check
    (if (Variables|/Game/QTE/BP_QTEManager.BP_QTEManager_C|GetHasPlayerWonQTE (Variables|Default|GetQTEManager))
      ;[1 0.1661 0.9631] Won QTE
      (Utilities|FlowControl|DoOnce false
        (:Completed
          (CallFunction|TimeManipulation 0 (Variables|Default|GetGuards) 1.0 0.0)
          (Variables|Default|SetCustomTimeDilation 1.0)
          (Pawn|Components|CharacterMovement|DisableMovement (Variables|Character|GetCharacterMovement))
          (Collision|SetActorEnableCollision false)
          (Widget|RemovefromParent (Variables|Default|GetQTEWidget))
          (Development|PrintString "Takedown_AI")
          (Utilities|FlowControl|Delay 0.2)
          (CallFunction|TimeManipulation 0 (Variables|Default|GetGuards) 1.0 1.0)
          (Variables|/Game/QTE/BP_QTEManager.BP_QTEManager_C|SetHasPlayerWonQTE (Variables|Default|GetQTEManager) false)
          (Variables|Default|SetIsStartingQTE false)))
      (else
        ;[1 0.1661 0.9631] Countdown QTE
        (Utilities|FlowControl|Delay 1.0)
        (Math|Float|IncrementFloat (Variables|Default|GetTimer)
          (:%20%20
            (if (> (Variables|Default|GetTimer) (Variables|Default|GetMaxTime))
              ;[1 0.1661 0.9631] End QTE by losing
              (Utilities|FlowControl|DoOnce false
                (:Completed
                  (CallFunction|TimeManipulation 0 (Variables|Default|GetGuards) 1.0 1.0)
                  (Variables|Default|SetCustomTimeDilation 1.0)
                  (Pawn|Components|CharacterMovement|DisableMovement (Variables|/Script/Engine.Character|GetCharacterMovement (Variables|Default|GetPlayer)))
                  (Collision|SetActorEnableCollision (Variables|Default|GetPlayer) false)
                  (Widget|RemovefromParent (Variables|Default|GetQTEWidget))
                  (Development|PrintString "Takedown_morto")
                  (Development|PrintString "YouLose")
                  (Utilities|FlowControl|Delay 1.0)
                  (Game|OpenLevel(byName) "DefaultMap"))))))))
    (else
      ;[0.5441 0.4626 1] Player visibility
      (if (Variables|Default|GetIsPlayerVisible?)
        (bind _returnvalue_2 (|PlayerRange self (Variables|Default|GetIn%20Range%20Distance))
          (:true2
            (if (not _returnvalue_2)
              (Variables|Default|SetIsPlayerVisible? false)
              ;[0.551 1 0.5322] Stop Ai behaviour before QTE
              (bind _returnvalue_3 (|PlayerRange_2 self 1e+02)
                (:true2
                  (if (and (Variables|Default|GethasAlreadyShoot?) _returnvalue_3)
                    (Utilities|Casting|CastToAIController_Enemy _returnvalue)
                    (Components|Movement|StopMovementImmediately (Variables|Character|GetCharacterMovement))
                    (bind _asbp_character_controller (Utilities|Casting|CastToBp_CharacterController (Game|Player|GetPlayerPawn 0)))
                    (Variables|/Game/Character/Bp_CharacterController.Bp_CharacterController_C|SetisFighting? _asbp_character_controller false)
                    (Pawn|UnPossess _returnvalue)
                    ;[1 0.1661 0.9631] QTE time manipulation
                    (Variables|Default|SetIsStartingQTE true)
                    (CallFunction|TimeManipulation _asbp_character_controller (Variables|Default|GetGuards) 0.4 0.0)
                    (Variables|Default|SetCustomTimeDilation 0.2)
                    (Utilities|FlowControl|DoOnce false
                      (:Completed
                        ;[1 0.4987 0.5326] Create WidgetQTE
                        (bind _returnvalue_4 (UserInterface|CreateWidget "/Game/QTE/WB_QTE.WB_QTE_C"))
                        (UserInterface|Viewport|AddtoViewport _returnvalue_4 0)
                        ;[1 0.1661 0.9631] Increase QTE difficulty
                        (Variables|Default|SetQTEWidget _returnvalue_4)
                        (Variables|/Game/QTE/BP_QTEManager.BP_QTEManager_C|SetNumberOfTimePlayerSeen _qtemanager (+ (Variables|/Game/QTE/BP_QTEManager.BP_QTEManager_C|GetNumberOfTimePlayerSeen _qtemanager) 1))))))))))))))

(event EventBeginPlay
  ;[1 1 1] Get References
  (bind _returnvalue (Actor|GetActorOfClass "/Game/Character/Character_Build/BP_CharacterBuild.BP_CharacterBuild_C"))
  (Variables|Default|SetPlayer _returnvalue)
  (|GuardsRef)
  (|QTEManRef))

(fn ConstructionScript)

(fn TimeManipulation
  (params (Player :type Pawn%20Object%20Reference) (guard :type Array%20of%20BP%20AI%20Guards%20Object%20References) (PlayerTime :type Float%20%28single-precision%29) (GuardTime :type Float%20%28single-precision%29))
  (Variables|/Script/Engine.Actor|SetCustomTimeDilation Player PlayerTime)
  (for _array_element guard
    (Variables|/Script/Engine.Actor|SetCustomTimeDilation _array_element GuardTime)))