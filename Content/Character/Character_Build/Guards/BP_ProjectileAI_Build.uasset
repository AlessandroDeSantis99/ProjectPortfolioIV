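; BP_ProjectileAI_Build is a guard stun projectile that homes in on BP_CharacterBuild and freezes the player.
; Each tick, AimToPlayer moves it straight toward the player's current position at Speed, without sweeping.
; On overlap it freezes the player, plays a stun sound, clears StretchingManager's platform and projection, then destroys itself.
; BeginPlay also applies the same freeze and cleanup after a Duration delay, without destroying the projectile.
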(event OnComponentBeginOverlap(Sphere_Collision)
  (params (OverlappedComponent :type Primitive%20Component%20Object%20Reference) (OtherActor :type Actor%20Object%20Reference) (OtherComp :type Primitive%20Component%20Object%20Reference) (OtherBodyIndex :type Integer) (bFromSweep :type Boolean) (SweepResult :type Hit%20Result%20Structure%20%28by%20ref%29))
  (bind _stretchingmanager (Variables|Default|GetStretchingManager))
  (bind _asbp_character_build (Utilities|Casting|CastToBP_CharacterBuild OtherActor))
  (Variables|/Game/Character/Character_Build/BP_CharacterBuild.BP_CharacterBuild_C|SetQTEFrozen _asbp_character_build true)
  (Variables|/Game/Character/Character_Build/BP_CharacterBuild.BP_CharacterBuild_C|SetIsFrozen? _asbp_character_build true)
  (Audio|PlaySound2D "/Game/Audio/SFX/Belica/Stunnata/BelicaStunnata.BelicaStunnata" 1.0 1.0 0.0 0 0)
  (Default|DeletePlatform _stretchingmanager)
  (Default|DeleteProjection _stretchingmanager)
  (Actor|DestroyActor))

(event EventBeginPlay
  (Audio|PlaySound2D "/Game/Audio/SFX/rumori_cibernetici/PistolaStun.PistolaStun" 1.0 1.0 0.0 0 0)
  (bind _returnvalue (Actor|GetActorOfClass "/Game/Character/Character_Build/BP_CharacterBuild.BP_CharacterBuild_C"))
  (Variables|Default|SetPlayer _returnvalue)
  (bind _returnvalue_2 (Actor|GetActorOfClass "/Game/Strectching/BP_StretchingManager.BP_StretchingManager_C"))
  (Variables|Default|SetStretchingManager _returnvalue_2)
  (Utilities|FlowControl|Delay (Variables|Default|GetDuration))
  (Variables|/Game/Character/Character_Build/BP_CharacterBuild.BP_CharacterBuild_C|SetQTEFrozen (Variables|Default|GetPlayer) true)
  (Variables|/Game/Character/Character_Build/BP_CharacterBuild.BP_CharacterBuild_C|SetIsFrozen? (Variables|Default|GetPlayer) true)
  (Audio|PlaySound2D "/Game/Audio/SFX/Belica/Stunnata/BelicaStunnata.BelicaStunnata" 1.0 1.0 0.0 0 0)
  (Default|DeletePlatform (Variables|Default|GetStretchingManager))
  (Default|DeleteProjection (Variables|Default|GetStretchingManager)))

(event EventTick
  (params (DeltaSeconds :type Float%20%28single-precision%29))
  (CallFunction|AimtoPlayer (Variables|Default|GetSpeed) DeltaSeconds))

(fn ConstructionScript)

(fn AimtoPlayer
  (params (Speed :type Float%20%28single-precision%29) (DeltaTime :type Float%20%28single-precision%29))
  (Transformation|AddActorWorldOffset (* (* (Math|Vector|Normalize (- (Transformation|GetActorLocation (Variables|Default|GetPlayer)) (Transformation|GetActorLocation))) Speed) DeltaTime)))