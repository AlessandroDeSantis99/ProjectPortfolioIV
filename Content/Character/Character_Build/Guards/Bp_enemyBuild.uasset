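; Guard enemy character that detects the player by sight or hearing, shows an alert and can escalate into a close-range QTE fight.
; After shooting, a nearby guard triggers the QTE, using per-actor time dilation, a camera shift and a widget.
; Winning disables the guard, while timing out reopens the level.
; Tick also traces for BP_DirStretch obstacles that halt it, and an overlap area enables player takedowns.
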(event OnComponentBeginOverlap(TakedownArea)
  (params (OverlappedComponent :type Primitive%20Component%20Object%20Reference) (OtherActor :type Actor%20Object%20Reference) (OtherComp :type Primitive%20Component%20Object%20Reference) (OtherBodyIndex :type Integer) (bFromSweep :type Boolean) (SweepResult :type Hit%20Result%20Structure%20%28by%20ref%29))
  ;[1 0.7273 0.2762] Takedown
  (bind _asbp_character_build (Utilities|Casting|CastToBP_CharacterBuild OtherActor))
  (Variables|/Game/Character/Character_Build/BP_CharacterBuild.BP_CharacterBuild_C|SetCanTakedown? _asbp_character_build true))

(event OnComponentEndOverlap(TakedownArea)
  (params (OverlappedComponent :type Primitive%20Component%20Object%20Reference) (OtherActor :type Actor%20Object%20Reference) (OtherComp :type Primitive%20Component%20Object%20Reference) (OtherBodyIndex :type Integer))
  ;[1 0.7273 0.2762] Takedown
  (bind _asbp_character_build (Utilities|Casting|CastToBP_CharacterBuild OtherActor))
  (Variables|/Game/Character/Character_Build/BP_CharacterBuild.BP_CharacterBuild_C|SetCanTakedown? _asbp_character_build false))

(event OnSeePawn(PawnSensing)
  (params (Pawn :type Pawn%20Object%20Reference))
  ;[0.5441 0.4626 1] Has seen player
  (Variables|Default|SetIsPlayerVisible? true)
  ;[1 0.4987 0.5326] Exclamation mark
  (if (Variables|Default|GetIsPlayerSeenFirstTime?)
    (Variables|Default|SetIsPlayerSeenFirstTime? false)
    (Rendering|SetVisibility (Variables|Default|GetTextRender) true false)
    ;[0.551 1 0.5322] Allert stop
    (Components|Movement|StopMovementImmediately (Variables|Character|GetCharacterMovement))))

(event OnHearNoise(PawnSensing)
  (params (Instigator :type Pawn%20Object%20Reference) (Location :type Vector%20%28by%20ref%29 :default "0, 0, 0") (Volume :type Float%20%28single-precision%29))
  ;[0.5441 0.4626 1] Has heard player
  (Variables|Default|SetIsPlayerVisible? true)
  ;[1 0.4987 0.5326] Exclamation mark
  (if (Variables|Default|GetIsPlayerSeenFirstTime?)
    (Variables|Default|SetIsPlayerSeenFirstTime? false)
    (Rendering|SetVisibility (Variables|Default|GetTextRender) true false)
    ;[0.551 1 0.5322] Allert stop
    (Components|Movement|StopMovementImmediately (Variables|Character|GetCharacterMovement))))

(event Custom|Takedown
  ;[1 0.7273 0.2762] Takedown
  (Pawn|Components|CharacterMovement|DisableMovement (Variables|Character|GetCharacterMovement))
  (Collision|SetActorEnableCollision false)
  (Animation|PlayAnimMontage "/Game/ThirdPersonTemplateUnreal/Mannequin/Animations/CristodaroAnimation/Takedown_Montage/Takedown_Enemy.Takedown_Enemy" 1.0 "None"))

(event EventTick
  (params (DeltaSeconds :type Float%20%28single-precision%29))
  (bind _self self)
  (bind _capsulecomponent (Variables|Collision|GetCapsuleComponent))
  (bind _player (Variables|Default|GetPlayer))
  (bind _qtemanager (Variables|Default|GetQTEManager))
  (bind _capsulecomponent_2 (Variables|Collision|GetCapsuleComponent))
  (bind _returnvalue (Transformation|GetWorldLocation _capsulecomponent_2))
  (bind _returnvalue_2 (AI|GetAIController _self))
  (bind _returnvalue_3 (Transformation|GetWorldLocation _capsulecomponent))
  (bind _camera (Variables|/Game/Character/Character_Build/BP_CharacterBuild.BP_CharacterBuild_C|GetCamera _player))
  (if (or (Variables|Default|GetGo%20NearPlayer) (Variables|Default|GetIsStartingQTE))
    _
    (else
      (bind _outhit (Collision|LineTraceByChannel (Math|Vector|MakeVector (.x _returnvalue) (.y _returnvalue) (- (.z _returnvalue) 2e+01)) (+ (* (Math|Vector|GetForwardVector (Transformation|GetWorldRotation _capsulecomponent_2)) 1.1e+03) (Transformation|GetWorldLocation _capsulecomponent_2)) "TraceTypeQuery1" true 0 "ForOneFrame" true "(R=0.000000,G=0.355670,B=1.000000,A=1.000000)" "(R=1.000000,G=0.000000,B=0.839871,A=1.000000)"))
      (bind _asbp_dir_stretch (Utilities|Casting|CastToBP_DirStretch (.HitActor (Collision|BreakHitResult _outhit)))
        (:then
          (Variables|Default|SetHit%20Actor (.HitActor (Collision|BreakHitResult _outhit)))
          (CallFunction|InvisibilityCrouchWall _asbp_dir_stretch))
        (:CastFailed
          _))
      (bind _outhit_2 (Collision|LineTraceByChannel (Math|Vector|MakeVector (.x _returnvalue_3) (.y _returnvalue_3) (- (.z _returnvalue_3) 2e+01)) (+ (* (Math|Vector|GetForwardVector (Transformation|GetWorldRotation _capsulecomponent)) 5e+02) (Transformation|GetWorldLocation _capsulecomponent)) "TraceTypeQuery1" true 0 "ForOneFrame"))
      (Utilities|Casting|CastToBP_DirStretch (.HitActor (Collision|BreakHitResult _outhit_2))
        (:then
          (Variables|Default|SetHITPNC true)
          (Components|Movement|StopMovementImmediately (Variables|Character|GetCharacterMovement)))
        (:CastFailed
          _))
      (Utilities|IsValid (Variables|Default|GetHit%20Actor)
        (:Is%20Valid
          (if (< (.x (Transformation|GetActorScale3D (Variables|Default|GetHit%20Actor))) 0.8)
            (Variables|Default|SetHITPNC false)
            (Actor|DestroyActor (Variables|Default|GetHit%20Actor))))
        (:Is%20Not%20Valid
          _))))
  (if (Variables|Default|GetIsStartingQTE)
    ;[1 0.1661 0.9631] QTE check
    (if (Variables|/Game/QTE/BP_QTEManager.BP_QTEManager_C|GetHasPlayerWonQTE (Variables|Default|GetQTEManager))
      ;[1 0.1661 0.9631] Won QTE
      (Utilities|FlowControl|DoOnce false
        (:Completed
          (|RestartVelocity_player)
          (Variables|Default|SetCustomTimeDilation 1.0)
          (Pawn|Components|CharacterMovement|DisableMovement (Variables|Character|GetCharacterMovement))
          (Collision|SetActorEnableCollision false)
          (Widget|RemovefromParent (Variables|Default|GetQTEWidget))
          (Development|PrintString "Takedown_AI")
          (Utilities|FlowControl|Delay 0.2)
          (|RestartVelocity_General)
          (Variables|/Game/Character/Character_Build/BP_CharacterBuild.BP_CharacterBuild_C|SetIsFrozen? (Variables|Default|GetPlayer) false)
          (Variables|/Game/QTE/BP_QTEManager.BP_QTEManager_C|SetHasPlayerWonQTE (Variables|Default|GetQTEManager) false)
          (Variables|/Game/Character/Character_Build/BP_CharacterBuild.BP_CharacterBuild_C|SetIsFighting? (Variables|Default|GetPlayer) false)
          (Variables|Default|SetIsStartingQTE false)
          (Transformation|SetWorldLocation _camera (Variables|Default|GetLocationCamerPreQTE) false true)
          (Transformation|SetWorldRotation _camera (Variables|Default|GetRotationCameraPreQTE) false true)
          (Variables|/Game/Character/Character_Build/BP_CharacterBuild.BP_CharacterBuild_C|SetIsCameraFrozen? _player false)))
      (else
        ;[1 0.1661 0.9631] Countdown QTE
        (Utilities|FlowControl|Delay 1.0)
        (Math|Float|IncrementFloat (Variables|Default|GetTimer)
          (:%20%20
            (if (> (Variables|Default|GetTimer) (Variables|Default|GetMaxTime))
              ;[1 0.1661 0.9631] End QTE by losing
              (Utilities|FlowControl|DoOnce false
                (:Completed
                  (|RestartVelocity_General2)
                  (Variables|Default|SetCustomTimeDilation 1.0)
                  (Pawn|Components|CharacterMovement|DisableMovement (Variables|/Script/Engine.Character|GetCharacterMovement (Variables|Default|GetPlayer)))
                  (Collision|SetActorEnableCollision (Variables|Default|GetPlayer) false)
                  (Widget|RemovefromParent (Variables|Default|GetQTEWidget))
                  (Development|PrintString "Takedown_morto")
                  (Development|PrintString "YouLose")
                  (Utilities|FlowControl|Delay 1.0)
                  (Game|OpenLevel(byName) "Blockout_AlessandroDeSantis"))))))))
    (else
      ;[0.5441 0.4626 1] Player visibility
      (if (Variables|Default|GetIsPlayerVisible?)
        (bind _returnvalue_4 (|PlayerRange (Variables|Default|GetIn%20Range%20Distance))
          (:true2
            (if _returnvalue_4
              _
              (else
                (Variables|Default|SetIsPlayerVisible? false)))
            ;[0.551 1 0.5322] Stop Ai behaviour before QTE
            (bind _returnvalue_5 (|PlayerRange_2 1e+02)
              (:true2
                (if (and (Variables|Default|GethasAlreadyShoot?) _returnvalue_5)
                  (Utilities|Casting|CastToAIControllerEnemyBuild _returnvalue_2 :!label _label)
                  (Components|Movement|StopMovementImmediately (Variables|Character|GetCharacterMovement))
                  (Variables|/Game/Character/Character_Build/BP_CharacterBuild.BP_CharacterBuild_C|SetIsFighting? (Variables|Default|GetPlayer) true)
                  (Pawn|UnPossess _returnvalue_2)
                  ;[1 0.1661 0.9631] QTE time manipulation
                  (Variables|Default|SetIsStartingQTE true)
                  (|SlowDown)
                  (Utilities|FlowControl|DoOnce false
                    (:Completed
                      ;[1 1 1] CameraOrientation
                      (CallFunction|CameraOrientation self)
                      ;[1 0.4987 0.5326] Create WidgetQTE
                      (bind _returnvalue_6 (UserInterface|CreateWidget "/Game/QTE/WB_QTE.WB_QTE_C"))
                      (UserInterface|Viewport|AddtoViewport _returnvalue_6 0)
                      ;[1 0.1661 0.9631] Increase QTE difficulty
                      (Variables|Default|SetQTEWidget _returnvalue_6)
                      (Variables|/Game/QTE/BP_QTEManager.BP_QTEManager_C|SetNumberOfTimePlayerSeen _qtemanager (+ (Variables|/Game/QTE/BP_QTEManager.BP_QTEManager_C|GetNumberOfTimePlayerSeen _qtemanager) 1))))
                  (elif (and (Variables|Default|GethasAlreadyShoot?) (Variables|Default|GetIsStationary?))
                    (Variables|Default|SetGo%20NearPlayer true)
                    (bind _returnvalue_7 (|PlayerRange_2_2 1e+02)
                      (:true2
                        (if _returnvalue_7
                          (goto _label))))))))))))))

(event EventBeginPlay
  (bind _pawnsensing (Variables|Default|GetPawnSensing))
  ;[1 1 1] Get References
  (bind _returnvalue (Actor|GetActorOfClass "/Game/Character/Character_Build/BP_CharacterBuild.BP_CharacterBuild_C"))
  (Variables|Default|SetPlayer _returnvalue)
  (bind _outactors (Actor|GetAllActorsOfClass "Bp_enemyBuild_C"))
  (Variables|Default|SetGuards _outactors)
  (|QTEManRef)
  (Variables|/Script/AIModule.PawnSensingComponent|SetSightRadius _pawnsensing (Variables|Default|GetPawnSensingMaxDistance))
  (Variables|/Script/AIModule.PawnSensingComponent|SetHearingThreshold _pawnsensing (Variables|Default|GetPawnHearingMaxDistance)))

(fn ConstructionScript
  (Transformation|AttachComponentToComponent (Variables|Default|GetStaticMesh_Weapon) (Variables|Character|GetMesh) "Thumb_03_RSocket" "KeepRelative" "KeepRelative" "KeepRelative" true))

(fn TimeManipulation
  (params (Player :type Pawn%20Object%20Reference) (guard :type Array%20of%20BP%20AI%20Guards%20Object%20References) (PlayerTime :type Float%20%28single-precision%29) (GuardTime :type Float%20%28single-precision%29)))

(fn CameraOrientation
  (params (Enemy :type Bp%20Enemy%20Build%20Object%20Reference))
  (bind _player (Variables|Default|GetPlayer))
  (bind _camera (Variables|/Game/Character/Character_Build/BP_CharacterBuild.BP_CharacterBuild_C|GetCamera _player))
  (bind _scene_forward (Variables|/Game/Character/Character_Build/BP_CharacterBuild.BP_CharacterBuild_C|GetScene_Forward _player))
  (bind _scene_back (Variables|/Game/Character/Character_Build/BP_CharacterBuild.BP_CharacterBuild_C|GetScene_Back _player))
  (bind _capsulecomponent (Variables|/Script/Engine.Character|GetCapsuleComponent _player))
  (bind _returnvalue (Transformation|GetWorldLocation _scene_back))
  (bind _returnvalue_2 (Transformation|GetWorldLocation _scene_forward))
  (bind _returnvalue_3 (Transformation|GetWorldLocation _capsulecomponent))
  (Utilities|FlowControl|DoOnce false
    (:Completed
      (Variables|Default|SetLocationCamerPreQTE (Transformation|GetWorldLocation _camera))
      (Variables|Default|SetRotationCameraPreQTE (Transformation|GetWorldRotation _camera))
      (if (< (.x (- (Transformation|GetWorldLocation (Variables|/Script/Engine.Character|GetCapsuleComponent Enemy)) _returnvalue_3)) 0.0)
        (Transformation|SetWorldLocation _camera _returnvalue true false)
        (Transformation|SetWorldRotation _camera (Math|Rotator|FindLookatRotation _returnvalue _returnvalue_3) false true)
        (else
          (Transformation|SetWorldLocation _camera _returnvalue_2 true false)
          (Transformation|SetWorldRotation _camera (Math|Rotator|FindLookatRotation _returnvalue_2 _returnvalue_3) false true))))))

(fn InvisibilityCrouchWall
  (params (DirStretch :type BP%20Dir%20Stretch%20Object%20Reference))
  (bind _capsulecomponent (Variables|Collision|GetCapsuleComponent))
  (bind _returnvalue (Transformation|GetWorldLocation _capsulecomponent))
  (if (< (Math|Float|Absolute(Float) (Math|Vector|VectorLength (- _returnvalue (Transformation|GetWorldLocation (Variables|/Game/Strectching/BP_DirStretch.BP_DirStretch_C|GetInvisibilityCrouch_Forward DirStretch))))) (Math|Float|Absolute(Float) (Math|Vector|VectorLength (- _returnvalue (Transformation|GetWorldLocation (Variables|/Game/Strectching/BP_DirStretch.BP_DirStretch_C|GetInvisibilityCrouch_Back DirStretch))))))
    (Collision|SetCollisionEnabled (Variables|/Game/Strectching/BP_DirStretch.BP_DirStretch_C|GetInvisibilityCrouch_Back DirStretch) "QueryOnly")
    (else
      (Collision|SetCollisionEnabled (Variables|/Game/Strectching/BP_DirStretch.BP_DirStretch_C|GetInvisibilityCrouch_Forward DirStretch) "QueryOnly")))
  (return))