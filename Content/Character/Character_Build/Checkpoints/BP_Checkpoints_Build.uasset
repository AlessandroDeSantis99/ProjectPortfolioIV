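; Checkpoint actor that counts the build character's progress through a level, with each checkpoint usable only once.
; On overlap by BP_CharacterBuild it increments the count stored in a shared data asset and disables its collider.
; Shortly after BeginPlay, chained collapsed checks compare first, second and third "already taken" flags against its own identity booleans, disabling collision on matches.
; The data asset holds this state outside the actor; this Blueprint never sets those flags.
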(event OnComponentBeginOverlap(Collider)
  (params (OverlappedComponent :type Primitive%20Component%20Object%20Reference) (OtherActor :type Actor%20Object%20Reference) (OtherComp :type Primitive%20Component%20Object%20Reference) (OtherBodyIndex :type Integer) (bFromSweep :type Boolean) (SweepResult :type Hit%20Result%20Structure%20%28by%20ref%29))
  (Variables|Default|SetCurrentCheckpoint (Variables|/Game/Character/Character_Build/Checkpoints/DA_Checkpoint_Build.DA_Checkpoint_Build_C|GetCheckpoints (Variables|Default|GetDataAssetCheckpoint)))
  (Utilities|Casting|CastToBP_CharacterBuild OtherActor)
  ;[0.3838 0.4914 1] Checkpoint got
  (Math|Integer|IncrementInt (Variables|Default|GetCurrentCheckpoint)
    (:%20%20
      ;[1 0.4 0.402] Can't trigger checkpoint twice
      (Collision|SetCollisionEnabled (Variables|Default|GetCollider) "NoCollision")
      (Variables|/Game/Character/Character_Build/Checkpoints/DA_Checkpoint_Build.DA_Checkpoint_Build_C|SetCheckpoints (Variables|Default|GetDataAssetCheckpoint) (Variables|Default|GetCurrentCheckpoint)))))

(event EventBeginPlay
  (Utilities|FlowControl|Delay 0.2)
  ;[1 0.4 0.402] Can't trigger previous checkpoints
  (CallFunction|CheckPointTrigger))

(fn ConstructionScript)

(fn CheckPointTrigger
  (|FistCheckpointAlreadyTaken?
    (:then
      (|SecondCheckpointAlreadyTaken? :!label _label
        (:then2
          (|ThirdCheckpointAlreadyTaken? :!label _label_2))
        (:false
          (goto _label_2 false2))))
    (:false
      (goto _label false2))))