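; Checkpoint manager that places the BP_CharacterBuild player at its saved checkpoint when play begins.
; BeginPlay reads the checkpoint number from DataAssetCheckpoint and teleports the player to the matching SpawnPositions entry for checkpoints one to three.
; Each spawn also sets "already taken" flags on the data asset, though the third sets only the second and third flags.
; ResetCheckpointsCount zeroes the saved number, leaving the flags untouched.
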(event EventBeginPlay
  (bind _returnvalue (Actor|GetActorOfClass "/Game/Character/Character_Build/BP_CharacterBuild.BP_CharacterBuild_C"))
  (Variables|Default|SetPlayer _returnvalue)
  (CallFunction|SpawnPlayeratLocation (Variables|/Game/Character/Character_Build/DA_Checkpoint_Build.DA_Checkpoint_Build_C|GetCheckpoints (Variables|Default|GetDataAssetCheckpoint))))

(fn ConstructionScript)

(fn SpawnPlayeratLocation
  (params (CurrentCheckpoint :type Integer))
  (if (== CurrentCheckpoint 1)
    ;[0.4053 0.372 1] First Checkpoint
    (|SpawnAtFistCheckpoint)
    (elif (== CurrentCheckpoint 2)
      ;[0.4053 0.372 1] Second Checkpoint
      (|SpawnAtSecondLocation)
      (elif (== CurrentCheckpoint 3)
        ;[0.4053 0.372 1] ThirdCheckpoint
        (|SpawnAtThirdCheckpoint)))))

(fn ResetCheckpointsCount
  (Variables|/Game/Character/Character_Build/DA_Checkpoint_Build.DA_Checkpoint_Build_C|SetCheckpoints (Variables|Default|GetDataAssetCheckpoint) 0))