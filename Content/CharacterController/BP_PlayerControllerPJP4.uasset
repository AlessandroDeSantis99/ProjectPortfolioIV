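; BP_PlayerControllerPJP4 is a player controller that reads movement, look and jump input for the controlled pawn.
; Each axis event passes its value to the pawn as a message call, with separate calls for mouse and gamepad turn and look rates.
; Jump press and release set an IsJumping flag and send it to the pawn, leaving the response to each input up to the pawn.
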(event Input|ActionEvents|InputActionJump
  (params (Key :type Key%20Structure :default "None"))
  ;[1 0.3279 0.9465] Jumping input
  (:Pressed
    (bind _output_get (Variables|Default|SetIsJumping? true))
    (Class|IPlayerInputs|Jumping(Message) (Pawn|GetControlledPawn) _output_get))
  (:Released
    (bind _output_get_2 (Variables|Default|SetIsJumping? false))
    (Class|IPlayerInputs|Jumping(Message) (Pawn|GetControlledPawn) _output_get_2)))

(event Input|AxisEvents|InputAxisLookUp
  (params (AxisValue :type Float%20%28single-precision%29))
  ;[1 0.249 0.3828] Look up mouse input
  (Class|IPlayerInputs|LookUpRateMouse(Message) (Pawn|GetControlledPawn) AxisValue))

(event Input|AxisEvents|InputAxisTurnRate
  (params (AxisValue :type Float%20%28single-precision%29))
  ;[0.7768 1 0.6173] TurnRate gamepad input
  (Class|IPlayerInputs|TurnRateGamePad(Message) (Pawn|GetControlledPawn) AxisValue))

(event Input|AxisEvents|InputAxisTurn
  (params (AxisValue :type Float%20%28single-precision%29))
  ;[1 0.249 0.3828] TurnRate mouse input
  (Class|IPlayerInputs|TurnRateMouse(Message) (Pawn|GetControlledPawn) AxisValue))

(event Input|AxisEvents|InputAxisLookUpRate
  (params (AxisValue :type Float%20%28single-precision%29))
  ;[0.7768 1 0.6173] LookUp gamedpad input
  (Class|IPlayerInputs|LookUpRateGamePad(Message) (Pawn|GetControlledPawn) AxisValue))

(event Input|AxisEvents|InputAxisMoveForward
  (params (AxisValue :type Float%20%28single-precision%29))
  ;[0.4297 0.4055 1] Moving forward input
  (Class|IPlayerInputs|MoveForward(Message) (Pawn|GetControlledPawn) AxisValue))

(event Input|AxisEvents|InputAxisMoveRight
  (params (AxisValue :type Float%20%28single-precision%29))
  ;[0.3502 0.5 1] Moving right input
  (Class|IPlayerInputs|MoveRight(Message) (Pawn|GetControlledPawn) AxisValue))

(fn ConstructionScript)