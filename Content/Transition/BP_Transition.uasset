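; BP_Transition is a one-shot trigger that carries the player's mana into saved data and starts a screen fade.
; When BP_CharacterBuild overlaps its Box, it writes the character's Mana to the GI_SaveData game instance, raising it to a minimum of four.
; It then sets IsFading and adds a WD_Fader widget to the viewport; no level load happens in this Blueprint.
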(event OnComponentBeginOverlap(Box)
  (params (OverlappedComponent :type Primitive%20Component%20Object%20Reference) (OtherActor :type Actor%20Object%20Reference) (OtherComp :type Primitive%20Component%20Object%20Reference) (OtherBodyIndex :type Integer) (bFromSweep :type Boolean) (SweepResult :type Hit%20Result%20Structure%20%28by%20ref%29))
  (bind _asbp_character_build (Utilities|Casting|CastToBP_CharacterBuild OtherActor))
  (Utilities|FlowControl|DoOnce false
    (:Completed
      (bind _asgi_save_data (Utilities|Casting|CastToGI_SaveData (Game|GetGameInstance)))
      (bind _output_get (Variables|Default|SetGameIstance _asgi_save_data))
      (if (< (Variables|/Game/Character/Character_Build/BP_CharacterBuild.BP_CharacterBuild_C|GetMana _asbp_character_build) 4.0)
        (Variables|/Game/Saving/GI_SaveData.GI_SaveData_C|SetMana _output_get 4.0)
        (Variables|Default|SetIsFading? true)
        (bind _returnvalue (UserInterface|CreateWidget "/Game/Transition/WD_Fader.WD_Fader_C"))
        (UserInterface|Viewport|AddtoViewport _returnvalue 0)
        (else
          (Variables|/Game/Saving/GI_SaveData.GI_SaveData_C|SetMana _asgi_save_data (Variables|/Game/Character/Character_Build/BP_CharacterBuild.BP_CharacterBuild_C|GetMana _asbp_character_build))
          (Variables|Default|SetIsFading? true)
          (bind _returnvalue_2 (UserInterface|CreateWidget "/Game/Transition/WD_Fader.WD_Fader_C"))
          (UserInterface|Viewport|AddtoViewport _returnvalue_2 0))))))

(fn ConstructionScript)