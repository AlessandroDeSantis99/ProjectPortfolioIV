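; Checkpoint trigger actor that counts player progress in a shared checkpoint data asset and can fire only once.
; Overlap by Bp_CharacterController increments the asset's checkpoint count and disables the collider.
; On BeginPlay, chained checks pair the instance's first, second or third flag with the asset's "already taken" flags, disabling colliders of earlier checkpoints.
; The taken flags are only read here, never set.
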(event OnComponentBeginOverlap(Collider)
  (params (OverlappedComponent :type Primitive%20Component%20Object%20Reference) (OtherActor :type Actor%20Object%20Reference) (OtherComp :type Primitive%20Component%20Object%20Reference) (OtherBodyIndex :type Integer) (bFromSweep :type Boolean) (SweepResult :type Hit%20Result%20Structure%20%28by%20ref%29))
  (Variables|Default|SetCurrentCheckpoint (Variables|/Game/CheckPoints/DA_Checkpoint.DA_Checkpoint_C|GetCheckpoints (Variables|Default|GetDataAssetCheckpoint)))
  (Utilities|Casting|CastToBp_CharacterController OtherActor)
  (bind _result (Math|Integer|IncrementInt (Variables|Default|GetCurrentCheckpoint))
    (:%20%20
      ;[1 0.4 0.402] Can't trigger checkpoint twice
      (Collision|SetCollisionEnabled (Variables|Default|GetCollider) "NoCollision")
      (Variables|/Game/CheckPoints/DA_Checkpoint.DA_Checkpoint_C|SetCheckpoints (Variables|Default|GetDataAssetCheckpoint) _result))))

(event EventBeginPlay
  ;[1 0.4 0.402] Can't trigger previous checkpoints
  (CallFunction|CheckPointTrigger))

(fn ConstructionScript)

(fn CheckPointTrigger
  (|FistCheckpointAlreadyTaken?
    (:then
      (|SecondCheckpointAlreadyTaken :!label _label
        (:then2
          (|ThirdCheckpointAlreadyTaken_2 :!label _label_2))
        (:false
          (goto _label_2 false2))))
    (:false
      (goto _label false2))))