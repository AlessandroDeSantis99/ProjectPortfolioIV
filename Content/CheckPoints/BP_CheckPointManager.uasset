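; Checkpoint manager that moves the player to the last saved checkpoint when play begins.
; It reads the checkpoint number from a checkpoint data asset and teleports the player to the matching entry in SpawnPositions, supporting three checkpoints.
; Each spawn also flags that checkpoint and all earlier ones as taken in the data asset.
; A separate function resets the stored count to zero, for which no teleport occurs.
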(event EventBeginPlay
  (bind _playeristance (CallFunction|GetPlayerIstance))
  (Variables|Default|SetPlayer _playeristance)
  (CallFunction|SpawnPlayeratLocation (Variables|/Game/CheckPoints/DA_Checkpoint.DA_Checkpoint_C|GetCheckpoints (Variables|Default|GetDataAssetCheckpoint))))

(fn ConstructionScript)

(fn SpawnPlayeratLocation
  (params (CurrentCheckpoint :type Integer))
  (if (== CurrentCheckpoint 1)
    ;[0.4053 0.372 1] First Checkpoint
    (|SpawnAtFistCheckpoint)
    (elif (== CurrentCheckpoint 2)
      ;[0.4053 0.372 1] Second Checkpoint
      (|SpawnAtSecondLocation)
      (elif (== CurrentCheckpoint 3)
        ;[0.4053 0.372 1] ThirdCheckpoint
        (|SpawnAtThirdCheckpoint)))))

(fn ResetCheckpointsCount
  (Variables|/Game/CheckPoints/DA_Checkpoint.DA_Checkpoint_C|SetCheckpoints (Variables|Default|GetDataAssetCheckpoint) 0))