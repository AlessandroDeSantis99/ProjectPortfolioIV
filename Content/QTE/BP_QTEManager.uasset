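; BP_QTEManager relays quick-time-event input to the WB_QTE widget and supplies random keys from keyboard and joystick lists.
; Six QTE input actions send per-position key messages to the first top-level widget found, only when IsUsingController is true.
; When it is false, only the gamepad bottom face button forwards a first-key press; the other five branches are unwired.
; Both random pickers use array length as the inclusive maximum, one past the last index.
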(event Input|ActionEvents|InputActionQTE5
  (params (Key :type Key%20Structure :default "None"))
  (:Pressed
    (if (Variables|Default|GetIsUsingController?)
      (bind _widgetqte (CallFunction|GetWidgetQTE))
      (Class|IAIQTE|IsFifhtKeyPressed?(Message) _widgetqte Key))))

(event Input|ActionEvents|InputActionQTE6
  (params (Key :type Key%20Structure :default "None"))
  (:Pressed
    (if (Variables|Default|GetIsUsingController?)
      (bind _widgetqte (CallFunction|GetWidgetQTE))
      (Class|IAIQTE|IsSixthKeyPressed?(Message) _widgetqte Key))))

(event Input|ActionEvents|InputActionQTE
  (params (Key :type Key%20Structure :default "None"))
  (:Pressed
    (if (Variables|Default|GetIsUsingController?)
      (bind _widgetqte (CallFunction|GetWidgetQTE))
      (Class|IAIQTE|IsFirstKeyPressed?(Message) _widgetqte Key))))

(event Input|ActionEvents|InputActionQTE2
  (params (Key :type Key%20Structure :default "None"))
  (:Pressed
    (if (Variables|Default|GetIsUsingController?)
      (bind _widgetqte (CallFunction|GetWidgetQTE))
      (Class|IAIQTE|IsSecondKeyPressed?(Message) _widgetqte Key))))

(event Input|ActionEvents|InputActionQTE3
  (params (Key :type Key%20Structure :default "None"))
  (:Pressed
    (if (Variables|Default|GetIsUsingController?)
      (bind _widgetqte (CallFunction|GetWidgetQTE))
      (Class|IAIQTE|IsThirdKeyPressed?(Message) _widgetqte Key))))

(event Input|ActionEvents|InputActionQTE4
  (params (Key :type Key%20Structure :default "None"))
  (:Pressed
    (if (Variables|Default|GetIsUsingController?)
      (bind _widgetqte (CallFunction|GetWidgetQTE))
      (Class|IAIQTE|IsFourthKeyPressed?(Message) _widgetqte Key))))

(event Input|GamepadEvents|GamepadFaceButtonBottom
  (params (Key :type Key%20Structure :default "None"))
  (:Pressed
    (if (not (Variables|Default|GetIsUsingController?))
      (bind _widgetqte (CallFunction|GetWidgetQTE))
      (Class|IAIQTE|IsFirstKeyPressed?(Message) _widgetqte Key))))

(fn ConstructionScript)

(fn GetWidgetQTE
  (bind _foundwidgets (Widget|GetAllWidgetsOfClass "/Game/UI/Widgets/WB_QTE.WB_QTE_C" true))
  (return (Utilities|Array|Get(acopy) _foundwidgets)))

(fn GetKeyJoystick
  (return (Utilities|Array|Get(acopy) (Variables|Default|GetKeysJoystick) (Math|Random|RandomIntegerinRange 0 (Utilities|Array|Length (Variables|Default|GetKeysJoystick))))))

(fn GetKeyKeyboard
  (return (Utilities|Array|Get(acopy) (Variables|Default|GetKeys) (Math|Random|RandomIntegerinRange 0 (Utilities|Array|Length (Variables|Default|GetKeys))))))