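; Manager for the player's mana-based stretching ability, which extends poles ("Palo") and platforms on input, except while the player is fighting or frozen.
; Stretching spawns pole segments at growing offsets in the chosen one of four directions, or progressively larger copies of the looked-at platform, up to set limits.
; De-stretching undoes the latest piece (pole segments are shrunk, not destroyed) and refunds mana.
; AllDelete destroys all spawned pieces, refunds mana and resets counters.
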(event EventBeginPlay
  ;[1 1 1] References
  (bind _outactors (Actor|GetAllActorsOfClass "/Game/Strectching/BP_PaloStretchingDirection.BP_PaloStretchingDirection_C"))
  (Variables|Default|SetPaliDirection _outactors)
  (bind _returnvalue (Actor|GetActorOfClass "/Game/Character/Character_Build/BP_CharacterBuild.BP_CharacterBuild_C"))
  (Variables|Default|SetPlayer _returnvalue))

(event Input|ActionEvents|InputActionAllDelete
  (params (Key :type Key%20Structure :default "None"))
  (:Pressed
    (bind _outactors (Actor|GetAllActorsOfClass "/Game/Strectching/BP_Platform.BP_Platform_C"))
    (for _array_element _outactors
      (Utilities|IsValid _array_element
        (:Is%20Valid
          (Utilities|Array|Clear (Variables|/Game/Strectching/BP_Platform.BP_Platform_C|GetSpawnedPlatfroms _array_element))
          (Variables|/Game/Strectching/BP_Platform.BP_Platform_C|SetCurrentSpawnedPlatform _array_element 0)
          (Variables|/Game/Strectching/BP_Platform.BP_Platform_C|SetScale%20Platform _array_element "1.000000,1.000000,1.000000"))))
    (bind _outactors_2 (Actor|GetAllActorsOfClass "/Game/Strectching/BP_PlatformSpawned.BP_PlatformSpawned_C"))
    (for _array_element_2 _outactors_2
      (Utilities|IsValid _array_element_2
        (:Is%20Valid
          (Actor|DestroyActor _array_element_2)
          (Variables|/Game/Character/Character_Build/BP_CharacterBuild.BP_CharacterBuild_C|SetMana (Variables|Default|GetPlayer) (+ (Variables|/Game/Character/Character_Build/BP_CharacterBuild.BP_CharacterBuild_C|GetMana (Variables|Default|GetPlayer)) 1.0)))))))

(event Input|ActionEvents|InputActionStretchingPart
  (params (Key :type Key%20Structure :default "None"))
  (bind _player (Variables|Default|GetPlayer))
  (bind _player_2 (Variables|Default|GetPlayer))
  ;[1 1 1] Stretching
  (:Pressed
    (if (not (Variables|/Game/Character/Character_Build/BP_CharacterBuild.BP_CharacterBuild_C|GetIsFighting? (Variables|Default|GetPlayer)))
      (Variables|Default|SetUpperBody? true)
      (Animation|PlayAnimMontage (Variables|Default|GetPlayer) "/Game/MagicHeal_Montage.MagicHeal_Montage" 1.0 "None")
      (if (Variables|/Game/Character/Character_Build/BP_CharacterBuild.BP_CharacterBuild_C|GetIsLookingAtPlatform? _player)
        (if (not (Variables|/Game/Character/Character_Build/BP_CharacterBuild.BP_CharacterBuild_C|GetIsFrozen? _player))
          (CallFunction|SpawnPlatform _player_2))
        (elif (not (Variables|/Game/Character/Character_Build/BP_CharacterBuild.BP_CharacterBuild_C|GetIsFrozen? _player))
          (for _array_element (Variables|Default|GetPaliDirection)
            (if (Variables|/Game/Strectching/BP_PaloStretchingDirection.BP_PaloStretchingDirection_C|GetStartStretching? _array_element)
              (CallFunction|SpawnProjection _player_2 _array_element)))))))
  (:Released
    (for _array_element_2 (Variables|Default|GetPaliDirection)
      (Variables|/Game/Strectching/BP_PaloStretchingDirection.BP_PaloStretchingDirection_C|SetStartStretching? _array_element_2 false))))

(event Input|ActionEvents|InputActionDeStretchingPart
  (params (Key :type Key%20Structure :default "None"))
  (bind _player (Variables|Default|GetPlayer))
  (bind _player_2 (Variables|Default|GetPlayer))
  ;[1 1 1] De Stretching
  (:Pressed
    (if (not (Variables|/Game/Character/Character_Build/BP_CharacterBuild.BP_CharacterBuild_C|GetIsFighting? (Variables|Default|GetPlayer)))
      (Variables|Default|SetUpperBody? true)
      (Animation|PlayAnimMontage (Variables|Default|GetPlayer) "/Game/MagicHeal_Montage.MagicHeal_Montage" 1.0 "None")
      (if (Variables|/Game/Character/Character_Build/BP_CharacterBuild.BP_CharacterBuild_C|GetIsLookingAtPlatform? _player)
        (if (not (Variables|/Game/Character/Character_Build/BP_CharacterBuild.BP_CharacterBuild_C|GetIsFrozen? _player))
          (CallFunction|DeSpawnPlatform _player_2))
        (elif (not (Variables|/Game/Character/Character_Build/BP_CharacterBuild.BP_CharacterBuild_C|GetIsFrozen? _player))
          (for _array_element (Variables|Default|GetPaliDirection)
            (if (Variables|/Game/Strectching/BP_PaloStretchingDirection.BP_PaloStretchingDirection_C|GetStartStretching? _array_element)
              (CallFunction|DeSpawnProjection _player_2 _array_element)))))))
  (:Released
    (for _array_element_2 (Variables|Default|GetPaliDirection)
      (Variables|/Game/Strectching/BP_PaloStretchingDirection.BP_PaloStretchingDirection_C|SetStartStretching? _array_element_2 false))))

(event Input|ActionEvents|InputActionAllDelete
  (params (Key :type Key%20Structure :default "None"))
  (bind _player (Variables|Default|GetPlayer))
  (bind _as_bp_palo_stretching_direction (Variables|/Game/Character/Character_Build/BP_CharacterBuild.BP_CharacterBuild_C|GetAs%20BP%20Palo%20Stretching%20Direction _player))
  (bind _dirsstretch_0 (Variables|/Game/Strectching/BP_PaloStretchingDirection.BP_PaloStretchingDirection_C|GetDirsStretch_0 _as_bp_palo_stretching_direction))
  (bind _dirsstretch_1 (Variables|/Game/Strectching/BP_PaloStretchingDirection.BP_PaloStretchingDirection_C|GetDirsStretch_1 _as_bp_palo_stretching_direction))
  (bind _dirsstretch_2 (Variables|/Game/Strectching/BP_PaloStretchingDirection.BP_PaloStretchingDirection_C|GetDirsStretch_2 _as_bp_palo_stretching_direction))
  (:Pressed
    (bind _outactors (Actor|GetAllActorsOfClass "/Game/Strectching/BP_DirStretch.BP_DirStretch_C"))
    (bind _output_get (Variables|Default|SetPaliSpawnati _outactors))
    (for _array_element (Variables|Default|GetPaliDirection)
      (Variables|/Game/Strectching/BP_PaloStretchingDirection.BP_PaloStretchingDirection_C|SetSpawnDistance_0 _array_element 0.0)
      (Variables|/Game/Strectching/BP_PaloStretchingDirection.BP_PaloStretchingDirection_C|SetSpawnDistance_1 _array_element 0.0)
      (Variables|/Game/Strectching/BP_PaloStretchingDirection.BP_PaloStretchingDirection_C|SetSpawnDistance_3 _array_element 0.0)
      (Variables|/Game/Strectching/BP_PaloStretchingDirection.BP_PaloStretchingDirection_C|SetSpawnDistance_2 _array_element 0.0))
    (Utilities|IsValid _as_bp_palo_stretching_direction
      (:Is%20Valid
        (if (> (Utilities|Array|Length _dirsstretch_0) 0)
          (Utilities|Array|Clear _dirsstretch_0))
        (if (> (Utilities|Array|Length _dirsstretch_1) 0)
          (Utilities|Array|Clear _dirsstretch_1))
        (if (> (Utilities|Array|Length _dirsstretch_2) 0)
          (Utilities|Array|Clear _dirsstretch_2))
        (if true
          (Utilities|Array|Clear (Variables|/Game/Strectching/BP_PaloStretchingDirection.BP_PaloStretchingDirection_C|GetDirsStretch_3 _as_bp_palo_stretching_direction)))
        (for _array_element_2 _output_get
          (Utilities|IsValid _array_element_2
            (:Is%20Valid
              (Actor|DestroyActor _array_element_2)
              (Variables|/Game/Character/Character_Build/BP_CharacterBuild.BP_CharacterBuild_C|SetMana (Variables|Default|GetPlayer) (+ (Variables|/Game/Character/Character_Build/BP_CharacterBuild.BP_CharacterBuild_C|GetMana (Variables|Default|GetPlayer)) 1.0))
              (Variables|Default|SetSpawnQuantity_3 0)
              (Variables|Default|SetSpawnQuantity_1 0)
              (Variables|Default|SetSpawnQuantity_2 0)
              (Variables|Default|SetSpawnQuantity_0 0))))))))

(fn ConstructionScript)

(fn DisableOthersPali
  (params (lookedPalo :type BP%20Palo%20Stretching%20Direction%20Object%20Reference))
  (for _array_element (Variables|Default|GetPaliDirection)
    (Actor|Tick|SetActorTickEnabled _array_element)
    (Rendering|SetVisibility (Variables|/Game/Strectching/BP_PaloStretchingDirection.BP_PaloStretchingDirection_C|GetWidget _array_element) false false)
    (Actor|Tick|SetActorTickEnabled lookedPalo true)))

(fn EnableOthersPali
  (for _array_element (Variables|Default|GetPaliDirection)
    (Actor|Tick|SetActorTickEnabled _array_element true)))

(fn SpawnProjection
  (params (CharacterController :type BP%20Character%20Build%20Object%20Reference) (Palo :type BP%20Palo%20Stretching%20Direction%20Object%20Reference))
  (bind _canpreviewdir2 (Variables|/Game/Strectching/BP_PaloStretchingDirection.BP_PaloStretchingDirection_C|GetCanPreviewDir2 Palo))
  (bind _canpreviewdir3 (Variables|/Game/Strectching/BP_PaloStretchingDirection.BP_PaloStretchingDirection_C|GetCanPreviewDir3 Palo))
  (bind _canpreviewdir4 (Variables|/Game/Strectching/BP_PaloStretchingDirection.BP_PaloStretchingDirection_C|GetCanPreviewDir4 Palo))
  (bind _palo_steatch_dir_1 (Variables|/Game/Character/Character_Build/BP_CharacterBuild.BP_CharacterBuild_C|GetPalo%20Steatch%20Dir_1 CharacterController))
  (bind _palo_steatch_dir_2 (Variables|/Game/Character/Character_Build/BP_CharacterBuild.BP_CharacterBuild_C|GetPalo%20Steatch%20Dir_2 CharacterController))
  (bind _player (Variables|Default|GetPlayer))
  (bind _palo_steatch_dir_3 (Variables|/Game/Character/Character_Build/BP_CharacterBuild.BP_CharacterBuild_C|GetPalo%20Steatch%20Dir_3 CharacterController))
  (bind _palo_steatch_dir_4_ (Variables|/Game/Character/Character_Build/BP_CharacterBuild.BP_CharacterBuild_C|GetPalo%20Steatch%20Dir_4%20 CharacterController))
  (bind _returnvalue (Transformation|GetWorldLocation _palo_steatch_dir_2))
  (bind _returnvalue_2 (Transformation|GetWorldLocation _palo_steatch_dir_1))
  (bind _returnvalue_3 (Transformation|GetWorldLocation _palo_steatch_dir_3))
  (bind _returnvalue_4 (Transformation|GetWorldLocation _palo_steatch_dir_4_))
  (bind _dirtostretch (Variables|/Game/Character/Character_Build/BP_CharacterBuild.BP_CharacterBuild_C|GetDirToStretch _player))
  (if (Variables|/Game/Strectching/BP_PaloStretchingDirection.BP_PaloStretchingDirection_C|GetCanPreviewDir1 Palo)
    (Utilities|IsValid _palo_steatch_dir_1
      (:Is%20Valid
        (if (== _palo_steatch_dir_1 _dirtostretch)
          (if (> (Variables|/Game/Character/Character_Build/BP_CharacterBuild.BP_CharacterBuild_C|GetMana (Variables|Default|GetPlayer)) 0.1)
            (if (< (Variables|Default|GetSpawnQuantity_0) (Variables|/Game/Strectching/BP_PaloStretchingDirection.BP_PaloStretchingDirection_C|GetMaxSpawnDir1 Palo))
              (bind _returnvalue_5 (Game|SpawnActorfromClass "/Game/Strectching/BP_DirStretch.BP_DirStretch_C" (Math|Transform|MakeTransform (Math|Vector|MakeVector (- (.x _returnvalue_2) (Variables|/Game/Strectching/BP_PaloStretchingDirection.BP_PaloStretchingDirection_C|GetSpawnDistance_0 Palo)) (.y _returnvalue_2) (.z _returnvalue_2)) (Transformation|GetWorldRotation (Variables|/Game/Character/Character_Build/BP_CharacterBuild.BP_CharacterBuild_C|GetArrowDirToStretch (Variables|Default|GetPlayer))) "1,1,1") "Undefined" 0 0))
              (Utilities|Array|Add (Variables|Default|GetDirStretch_0) _returnvalue_5)
              (Variables|/Game/Strectching/BP_PaloStretchingDirection.BP_PaloStretchingDirection_C|SetSpawnDistance_0 Palo (+ (Variables|/Game/Strectching/BP_PaloStretchingDirection.BP_PaloStretchingDirection_C|GetSpawnDistance_0 Palo) (Variables|Default|GetAdd%20spawn%20distance_0)))
              (Variables|/Game/Character/Character_Build/BP_CharacterBuild.BP_CharacterBuild_C|SetMana (Variables|Default|GetPlayer) (- (Variables|/Game/Character/Character_Build/BP_CharacterBuild.BP_CharacterBuild_C|GetMana (Variables|Default|GetPlayer)) 1.0))
              (Math|Integer|IncrementInt (Variables|Default|GetSpawnQuantity_0))))
          (else
            (if _canpreviewdir2 :!label _label
              (Utilities|IsValid _palo_steatch_dir_2 :!label _label_2
                (:Is%20Valid
                  (if (== _palo_steatch_dir_2 _dirtostretch)
                    (if (> (Variables|/Game/Character/Character_Build/BP_CharacterBuild.BP_CharacterBuild_C|GetMana (Variables|Default|GetPlayer)) 0.1)
                      (if (< (Variables|Default|GetSpawnQuantity_1) (Variables|/Game/Strectching/BP_PaloStretchingDirection.BP_PaloStretchingDirection_C|GetMaxSpawnDir2 Palo))
                        (bind _returnvalue_6 (Game|SpawnActorfromClass "/Game/Strectching/BP_DirStretch.BP_DirStretch_C" (Math|Transform|MakeTransform (Math|Vector|MakeVector (+ (Variables|/Game/Strectching/BP_PaloStretchingDirection.BP_PaloStretchingDirection_C|GetSpawnDistance_1 Palo) (.x _returnvalue)) (.y _returnvalue) (.z _returnvalue)) (Transformation|GetWorldRotation (Variables|/Game/Character/Character_Build/BP_CharacterBuild.BP_CharacterBuild_C|GetArrowDirToStretch (Variables|Default|GetPlayer))) "1,1,1") "Undefined" 0 0))
                        (Utilities|Array|Add (Variables|Default|GetDirStretch_1) _returnvalue_6)
                        (Variables|/Game/Strectching/BP_PaloStretchingDirection.BP_PaloStretchingDirection_C|SetSpawnDistance_1 Palo (+ (Variables|/Game/Strectching/BP_PaloStretchingDirection.BP_PaloStretchingDirection_C|GetSpawnDistance_1 Palo) (Variables|Default|GetAdd%20spawn%20distance_0)))
                        (Variables|/Game/Character/Character_Build/BP_CharacterBuild.BP_CharacterBuild_C|SetMana (Variables|Default|GetPlayer) (- (Variables|/Game/Character/Character_Build/BP_CharacterBuild.BP_CharacterBuild_C|GetMana (Variables|Default|GetPlayer)) 1.0))
                        (Math|Integer|IncrementInt (Variables|Default|GetSpawnQuantity_1))))
                    (else
                      (if _canpreviewdir3 :!label _label_3
                        (Utilities|IsValid _palo_steatch_dir_3 :!label _label_4
                          (:Is%20Valid
                            (if (== _palo_steatch_dir_3 _dirtostretch)
                              (if (> (Variables|/Game/Character/Character_Build/BP_CharacterBuild.BP_CharacterBuild_C|GetMana (Variables|Default|GetPlayer)) 0.1)
                                (if (< (Variables|Default|GetSpawnQuantity_2) (Variables|/Game/Strectching/BP_PaloStretchingDirection.BP_PaloStretchingDirection_C|GetMaxSpawnDir3 Palo))
                                  (bind _returnvalue_7 (Game|SpawnActorfromClass "/Game/Strectching/BP_DirStretch.BP_DirStretch_C" (Math|Transform|MakeTransform (Math|Vector|MakeVector (.x _returnvalue_3) (- (.y _returnvalue_3) (Variables|/Game/Strectching/BP_PaloStretchingDirection.BP_PaloStretchingDirection_C|GetSpawnDistance_2 Palo)) (.z _returnvalue_3)) (Transformation|GetWorldRotation (Variables|/Game/Character/Character_Build/BP_CharacterBuild.BP_CharacterBuild_C|GetArrowDirToStretch (Variables|Default|GetPlayer))) "1,1,1") "Undefined" 0 0))
                                  (Utilities|Array|Add (Variables|Default|GetDirStretch_2) _returnvalue_7)
                                  (Variables|/Game/Strectching/BP_PaloStretchingDirection.BP_PaloStretchingDirection_C|SetSpawnDistance_2 Palo (+ (Variables|Default|GetAdd%20spawn%20distance_0) (Variables|/Game/Strectching/BP_PaloStretchingDirection.BP_PaloStretchingDirection_C|GetSpawnDistance_2 Palo)))
                                  (Variables|/Game/Character/Character_Build/BP_CharacterBuild.BP_CharacterBuild_C|SetMana (Variables|Default|GetPlayer) (- (Variables|/Game/Character/Character_Build/BP_CharacterBuild.BP_CharacterBuild_C|GetMana (Variables|Default|GetPlayer)) 1.0))
                                  (Math|Integer|IncrementInt (Variables|Default|GetSpawnQuantity_2))))
                              (else
                                (if _canpreviewdir4 :!label _label_5
                                  (Utilities|IsValid _palo_steatch_dir_4_ :!label _label_6
                                    (:Is%20Valid
                                      (if (== _palo_steatch_dir_4_ _dirtostretch)
                                        (if (> (Variables|/Game/Character/Character_Build/BP_CharacterBuild.BP_CharacterBuild_C|GetMana (Variables|Default|GetPlayer)) 0.1)
                                          (if (< (Variables|Default|GetSpawnQuantity_3) (Variables|/Game/Strectching/BP_PaloStretchingDirection.BP_PaloStretchingDirection_C|GetMaxSpawnDir4 Palo))
                                            (bind _returnvalue_8 (Game|SpawnActorfromClass "/Game/Strectching/BP_DirStretch.BP_DirStretch_C" (Math|Transform|MakeTransform (Math|Vector|MakeVector (.x _returnvalue_4) (+ (Variables|/Game/Strectching/BP_PaloStretchingDirection.BP_PaloStretchingDirection_C|GetSpawnDistance_3 Palo) (.y _returnvalue_4)) (.z _returnvalue_4)) (Transformation|GetWorldRotation (Variables|/Game/Character/Character_Build/BP_CharacterBuild.BP_CharacterBuild_C|GetArrowDirToStretch (Variables|Default|GetPlayer))) "1,1,1") "Undefined" 0 0))
                                            (Utilities|Array|Add (Variables|Default|GetDirStretch_3) _returnvalue_8)
                                            (Variables|/Game/Strectching/BP_PaloStretchingDirection.BP_PaloStretchingDirection_C|SetSpawnDistance_3 Palo (+ (Variables|/Game/Strectching/BP_PaloStretchingDirection.BP_PaloStretchingDirection_C|GetSpawnDistance_3 Palo) (Variables|Default|GetAdd%20spawn%20distance_0)))
                                            (Variables|/Game/Character/Character_Build/BP_CharacterBuild.BP_CharacterBuild_C|SetMana (Variables|Default|GetPlayer) (- (Variables|/Game/Character/Character_Build/BP_CharacterBuild.BP_CharacterBuild_C|GetMana (Variables|Default|GetPlayer)) 1.0))
                                            (Math|Integer|IncrementInt (Variables|Default|GetSpawnQuantity_3)))))))))))
                          (:Is%20Not%20Valid
                            (goto _label_5)))
                        (else
                          (goto _label_5))))))
                (:Is%20Not%20Valid
                  (goto _label_3)))
              (else
                (goto _label_3))))))
      (:Is%20Not%20Valid
        (goto _label)))
    (elif _canpreviewdir2
      (goto _label_2)
      (elif _canpreviewdir3
        (goto _label_4)
        (elif _canpreviewdir4
          (goto _label_6))))))

(fn DeSpawnProjection
  (params (CharacterController :type BP%20Character%20Build%20Object%20Reference) (Palo :type BP%20Palo%20Stretching%20Direction%20Object%20Reference))
  (bind _player (Variables|Default|GetPlayer))
  (bind _player_2 (Variables|Default|GetPlayer))
  (bind _player_3 (Variables|Default|GetPlayer))
  (bind _player_4 (Variables|Default|GetPlayer))
  (bind _player_5 (Variables|Default|GetPlayer))
  (bind _as_bp_palo_stretching_direction (Variables|/Game/Character/Character_Build/BP_CharacterBuild.BP_CharacterBuild_C|GetAs%20BP%20Palo%20Stretching%20Direction _player))
  (bind _as_bp_palo_stretching_direction_2 (Variables|/Game/Character/Character_Build/BP_CharacterBuild.BP_CharacterBuild_C|GetAs%20BP%20Palo%20Stretching%20Direction _player_2))
  (bind _as_bp_palo_stretching_direction_3 (Variables|/Game/Character/Character_Build/BP_CharacterBuild.BP_CharacterBuild_C|GetAs%20BP%20Palo%20Stretching%20Direction _player_3))
  (bind _as_bp_palo_stretching_direction_4 (Variables|/Game/Character/Character_Build/BP_CharacterBuild.BP_CharacterBuild_C|GetAs%20BP%20Palo%20Stretching%20Direction _player_4))
  (bind _dirtostretch (Variables|/Game/Character/Character_Build/BP_CharacterBuild.BP_CharacterBuild_C|GetDirToStretch _player_5))
  (if (== (Variables|/Game/Character/Character_Build/BP_CharacterBuild.BP_CharacterBuild_C|GetPalo%20Steatch%20Dir_1 CharacterController) _dirtostretch)
    (Utilities|IsValid (Utilities|Array|Get(acopy) (Variables|/Game/Strectching/BP_PaloStretchingDirection.BP_PaloStretchingDirection_C|GetDirsStretch_0 _as_bp_palo_stretching_direction) (Utilities|Array|LastIndex (Variables|/Game/Strectching/BP_PaloStretchingDirection.BP_PaloStretchingDirection_C|GetDirsStretch_0 _as_bp_palo_stretching_direction)))
      (:Is%20Valid
        (Transformation|SetActorScale3D (Utilities|Array|Get(acopy) (Variables|/Game/Strectching/BP_PaloStretchingDirection.BP_PaloStretchingDirection_C|GetDirsStretch_0 _as_bp_palo_stretching_direction) (Utilities|Array|LastIndex (Variables|/Game/Strectching/BP_PaloStretchingDirection.BP_PaloStretchingDirection_C|GetDirsStretch_0 _as_bp_palo_stretching_direction))) "0.010000,0.010000,0.010000")
        (Utilities|Array|RemoveIndex (Variables|/Game/Strectching/BP_PaloStretchingDirection.BP_PaloStretchingDirection_C|GetDirsStretch_0 _as_bp_palo_stretching_direction) (Utilities|Array|LastIndex (Variables|/Game/Strectching/BP_PaloStretchingDirection.BP_PaloStretchingDirection_C|GetDirsStretch_0 _as_bp_palo_stretching_direction)))
        (Variables|/Game/Strectching/BP_PaloStretchingDirection.BP_PaloStretchingDirection_C|SetDirsStretch_0 _as_bp_palo_stretching_direction (Variables|/Game/Strectching/BP_PaloStretchingDirection.BP_PaloStretchingDirection_C|GetDirsStretch_0 _as_bp_palo_stretching_direction))
        (Variables|/Game/Strectching/BP_PaloStretchingDirection.BP_PaloStretchingDirection_C|SetSpawnDistance_0 Palo (- (Variables|/Game/Strectching/BP_PaloStretchingDirection.BP_PaloStretchingDirection_C|GetSpawnDistance_0 Palo) (Variables|Default|GetAdd%20spawn%20distance_0)))
        (Variables|/Game/Character/Character_Build/BP_CharacterBuild.BP_CharacterBuild_C|SetMana (Variables|Default|GetPlayer) (+ (Variables|/Game/Character/Character_Build/BP_CharacterBuild.BP_CharacterBuild_C|GetMana (Variables|Default|GetPlayer)) 1.0))
        (Math|Integer|DecrementInt (Variables|Default|GetSpawnQuantity_0))))
    (elif (== (Variables|/Game/Character/Character_Build/BP_CharacterBuild.BP_CharacterBuild_C|GetPalo%20Steatch%20Dir_2 CharacterController) _dirtostretch)
      (Utilities|IsValid (Utilities|Array|Get(acopy) (Variables|/Game/Strectching/BP_PaloStretchingDirection.BP_PaloStretchingDirection_C|GetDirsStretch_1 _as_bp_palo_stretching_direction_2) (Utilities|Array|LastIndex (Variables|/Game/Strectching/BP_PaloStretchingDirection.BP_PaloStretchingDirection_C|GetDirsStretch_1 _as_bp_palo_stretching_direction_2)))
        (:Is%20Valid
          (Transformation|SetActorScale3D (Utilities|Array|Get(acopy) (Variables|/Game/Strectching/BP_PaloStretchingDirection.BP_PaloStretchingDirection_C|GetDirsStretch_1 _as_bp_palo_stretching_direction_2) (Utilities|Array|LastIndex (Variables|/Game/Strectching/BP_PaloStretchingDirection.BP_PaloStretchingDirection_C|GetDirsStretch_1 _as_bp_palo_stretching_direction_2))) "0.010000,0.010000,0.010000")
          (Utilities|Array|RemoveIndex (Variables|/Game/Strectching/BP_PaloStretchingDirection.BP_PaloStretchingDirection_C|GetDirsStretch_1 _as_bp_palo_stretching_direction_2) (Utilities|Array|LastIndex (Variables|/Game/Strectching/BP_PaloStretchingDirection.BP_PaloStretchingDirection_C|GetDirsStretch_1 _as_bp_palo_stretching_direction_2)))
          (Variables|/Game/Strectching/BP_PaloStretchingDirection.BP_PaloStretchingDirection_C|SetDirsStretch_1 _as_bp_palo_stretching_direction_2 (Variables|/Game/Strectching/BP_PaloStretchingDirection.BP_PaloStretchingDirection_C|GetDirsStretch_1 _as_bp_palo_stretching_direction_2))
          (Variables|/Game/Strectching/BP_PaloStretchingDirection.BP_PaloStretchingDirection_C|SetSpawnDistance_1 Palo (- (Variables|/Game/Strectching/BP_PaloStretchingDirection.BP_PaloStretchingDirection_C|GetSpawnDistance_1 Palo) (Variables|Default|GetAdd%20spawn%20distance_0)))
          (Variables|/Game/Character/Character_Build/BP_CharacterBuild.BP_CharacterBuild_C|SetMana (Variables|Default|GetPlayer) (+ (Variables|/Game/Character/Character_Build/BP_CharacterBuild.BP_CharacterBuild_C|GetMana (Variables|Default|GetPlayer)) 1.0))
          (Math|Integer|DecrementInt (Variables|Default|GetSpawnQuantity_1))))
      (elif (== (Variables|/Game/Character/Character_Build/BP_CharacterBuild.BP_CharacterBuild_C|GetPalo%20Steatch%20Dir_3 CharacterController) _dirtostretch)
        (Utilities|IsValid (Utilities|Array|Get(acopy) (Variables|/Game/Strectching/BP_PaloStretchingDirection.BP_PaloStretchingDirection_C|GetDirsStretch_2 _as_bp_palo_stretching_direction_3) (Utilities|Array|LastIndex (Variables|/Game/Strectching/BP_PaloStretchingDirection.BP_PaloStretchingDirection_C|GetDirsStretch_2 _as_bp_palo_stretching_direction_3)))
          (:Is%20Valid
            (Transformation|SetActorScale3D (Utilities|Array|Get(acopy) (Variables|/Game/Strectching/BP_PaloStretchingDirection.BP_PaloStretchingDirection_C|GetDirsStretch_2 _as_bp_palo_stretching_direction_3) (Utilities|Array|LastIndex (Variables|/Game/Strectching/BP_PaloStretchingDirection.BP_PaloStretchingDirection_C|GetDirsStretch_2 _as_bp_palo_stretching_direction_3))) "0.010000,0.010000,0.010000")
            (Utilities|Array|RemoveIndex (Variables|/Game/Strectching/BP_PaloStretchingDirection.BP_PaloStretchingDirection_C|GetDirsStretch_2 _as_bp_palo_stretching_direction_3) (Utilities|Array|LastIndex (Variables|/Game/Strectching/BP_PaloStretchingDirection.BP_PaloStretchingDirection_C|GetDirsStretch_2 _as_bp_palo_stretching_direction_3)))
            (Variables|/Game/Strectching/BP_PaloStretchingDirection.BP_PaloStretchingDirection_C|SetDirsStretch_2 _as_bp_palo_stretching_direction_3 (Variables|/Game/Strectching/BP_PaloStretchingDirection.BP_PaloStretchingDirection_C|GetDirsStretch_2 _as_bp_palo_stretching_direction_3))
            (Variables|/Game/Strectching/BP_PaloStretchingDirection.BP_PaloStretchingDirection_C|SetSpawnDistance_2 Palo (- (Variables|/Game/Strectching/BP_PaloStretchingDirection.BP_PaloStretchingDirection_C|GetSpawnDistance_2 Palo) (Variables|Default|GetAdd%20spawn%20distance_0)))
            (Variables|/Game/Character/Character_Build/BP_CharacterBuild.BP_CharacterBuild_C|SetMana (Variables|Default|GetPlayer) (+ (Variables|/Game/Character/Character_Build/BP_CharacterBuild.BP_CharacterBuild_C|GetMana (Variables|Default|GetPlayer)) 1.0))
            (Math|Integer|DecrementInt (Variables|Default|GetSpawnQuantity_2))))
        (elif (== (Variables|/Game/Character/Character_Build/BP_CharacterBuild.BP_CharacterBuild_C|GetPalo%20Steatch%20Dir_4%20 CharacterController) _dirtostretch)
          (Utilities|IsValid (Utilities|Array|Get(acopy) (Variables|/Game/Strectching/BP_PaloStretchingDirection.BP_PaloStretchingDirection_C|GetDirsStretch_3 _as_bp_palo_stretching_direction_4) (Utilities|Array|LastIndex (Variables|/Game/Strectching/BP_PaloStretchingDirection.BP_PaloStretchingDirection_C|GetDirsStretch_3 _as_bp_palo_stretching_direction_4)))
            (:Is%20Valid
              (Transformation|SetActorScale3D (Utilities|Array|Get(acopy) (Variables|/Game/Strectching/BP_PaloStretchingDirection.BP_PaloStretchingDirection_C|GetDirsStretch_3 _as_bp_palo_stretching_direction_4) (Utilities|Array|LastIndex (Variables|/Game/Strectching/BP_PaloStretchingDirection.BP_PaloStretchingDirection_C|GetDirsStretch_3 _as_bp_palo_stretching_direction_4))) "0.010000,0.010000,0.010000")
              (Utilities|Array|RemoveIndex (Variables|/Game/Strectching/BP_PaloStretchingDirection.BP_PaloStretchingDirection_C|GetDirsStretch_3 _as_bp_palo_stretching_direction_4) (Utilities|Array|LastIndex (Variables|/Game/Strectching/BP_PaloStretchingDirection.BP_PaloStretchingDirection_C|GetDirsStretch_3 _as_bp_palo_stretching_direction_4)))
              (Variables|/Game/Strectching/BP_PaloStretchingDirection.BP_PaloStretchingDirection_C|SetDirsStretch_3 _as_bp_palo_stretching_direction_4 (Variables|/Game/Strectching/BP_PaloStretchingDirection.BP_PaloStretchingDirection_C|GetDirsStretch_3 _as_bp_palo_stretching_direction_4))
              (Variables|/Game/Strectching/BP_PaloStretchingDirection.BP_PaloStretchingDirection_C|SetSpawnDistance_3 Palo (- (Variables|/Game/Strectching/BP_PaloStretchingDirection.BP_PaloStretchingDirection_C|GetSpawnDistance_3 Palo) (Variables|Default|GetAdd%20spawn%20distance_0)))
              (Variables|/Game/Character/Character_Build/BP_CharacterBuild.BP_CharacterBuild_C|SetMana (Variables|Default|GetPlayer) (+ (Variables|/Game/Character/Character_Build/BP_CharacterBuild.BP_CharacterBuild_C|GetMana (Variables|Default|GetPlayer)) 1.0))
              (Math|Integer|DecrementInt (Variables|Default|GetSpawnQuantity_3))))
          (else
            (return)))))))

(fn SpawnPlatform
  (params (StretchingPlayer :type BP%20Character%20Build%20Object%20Reference))
  (bind _hittenplatform (Variables|/Game/Character/Character_Build/BP_CharacterBuild.BP_CharacterBuild_C|GetHittenPlatform StretchingPlayer))
  (bind _currentspawnedplatform (Variables|/Game/Strectching/BP_Platform.BP_Platform_C|GetCurrentSpawnedPlatform _hittenplatform))
  (bind _rootcomponent (Variables|/Script/Engine.Actor|GetRootComponent _hittenplatform))
  (bind _returnvalue (Transformation|GetWorldLocation _rootcomponent))
  (if (> (Variables|Default|GetMaxScalePlatform) _currentspawnedplatform)
    (bind _output_get (Variables|Default|SetPlatform%20scale (Variables|/Game/Strectching/BP_Platform.BP_Platform_C|GetScale%20Platform _hittenplatform)))
    (bind _returnvalue_2 (Game|SpawnActorfromClass "/Game/Strectching/BP_PlatformSpawned.BP_PlatformSpawned_C" (Math|Transform|MakeTransform (Math|Vector|MakeVector (.x _returnvalue) (.y _returnvalue) (.z _returnvalue)) "0, 0, 0" (Math|Vector|MakeVector (.x _output_get) (.y _output_get) (.z _output_get))) "Undefined" 0 0))
    (Utilities|Array|Add (Variables|/Game/Strectching/BP_Platform.BP_Platform_C|GetSpawnedPlatfroms _hittenplatform) _returnvalue_2)
    (Variables|/Game/Strectching/BP_Platform.BP_Platform_C|SetScale%20Platform _hittenplatform (Math|Vector|MakeVector (+ (.x (Variables|Default|GetPlatform%20scale)) 1.0) (.y (Variables|Default|GetPlatform%20scale)) (+ (.z (Variables|Default|GetPlatform%20scale)) 1.0)))
    (Variables|/Game/Character/Character_Build/BP_CharacterBuild.BP_CharacterBuild_C|SetMana (Variables|Default|GetPlayer) (- (Variables|/Game/Character/Character_Build/BP_CharacterBuild.BP_CharacterBuild_C|GetMana (Variables|Default|GetPlayer)) 1.0))
    (Math|Integer|IncrementInt _currentspawnedplatform)))

(fn DeSpawnPlatform
  (params (StretchingPlayer :type BP%20Character%20Build%20Object%20Reference))
  (bind _hittenplatform (Variables|/Game/Character/Character_Build/BP_CharacterBuild.BP_CharacterBuild_C|GetHittenPlatform StretchingPlayer))
  (bind _spawnedplatfroms (Variables|/Game/Strectching/BP_Platform.BP_Platform_C|GetSpawnedPlatfroms _hittenplatform))
  (bind _returnvalue (Utilities|Array|LastIndex _spawnedplatfroms))
  (bind _output (Utilities|Array|Get(acopy) _spawnedplatfroms _returnvalue))
  (Utilities|IsValid _output
    (:Is%20Valid
      (Actor|DestroyActor _output)
      (Utilities|Array|RemoveIndex _spawnedplatfroms _returnvalue)
      (Variables|/Game/Strectching/BP_Platform.BP_Platform_C|SetCurrentSpawnedPlatform _hittenplatform (- (Variables|/Game/Strectching/BP_Platform.BP_Platform_C|GetCurrentSpawnedPlatform _hittenplatform) 1))
      (Variables|/Game/Character/Character_Build/BP_CharacterBuild.BP_CharacterBuild_C|SetMana (Variables|Default|GetPlayer) (+ (Variables|/Game/Character/Character_Build/BP_CharacterBuild.BP_CharacterBuild_C|GetMana (Variables|Default|GetPlayer)) 1.0))
      (Variables|/Game/Strectching/BP_Platform.BP_Platform_C|SetScale%20Platform _hittenplatform (Math|Vector|MakeVector (- (.x (Variables|/Game/Strectching/BP_Platform.BP_Platform_C|GetScale%20Platform _hittenplatform)) 1.0) (.y (Variables|/Game/Strectching/BP_Platform.BP_Platform_C|GetScale%20Platform _hittenplatform)) (- (.z (Variables|/Game/Strectching/BP_Platform.BP_Platform_C|GetScale%20Platform _hittenplatform)) 1.0))))))

(fn DeSpawnPlatform0
  (params (StretchingPlayer :type BP%20Character%20Build%20Object%20Reference))
  (bind _hittenplatform (Variables|/Game/Character/Character_Build/BP_CharacterBuild.BP_CharacterBuild_C|GetHittenPlatform StretchingPlayer))
  (bind _spawnedplatfroms (Variables|/Game/Strectching/BP_Platform.BP_Platform_C|GetSpawnedPlatfroms _hittenplatform))
  (bind _returnvalue (Utilities|Array|LastIndex _spawnedplatfroms))
  (bind _output (Utilities|Array|Get(acopy) _spawnedplatfroms _returnvalue))
  (Utilities|IsValid _output
    (:Is%20Valid
      (Actor|DestroyActor _output)
      (Utilities|Array|RemoveIndex _spawnedplatfroms _returnvalue)
      (Variables|/Game/Strectching/BP_Platform.BP_Platform_C|SetCurrentSpawnedPlatform _hittenplatform (- (Variables|/Game/Strectching/BP_Platform.BP_Platform_C|GetCurrentSpawnedPlatform _hittenplatform) 1))
      (Variables|/Game/Character/Character_Build/BP_CharacterBuild.BP_CharacterBuild_C|SetMana (Variables|Default|GetPlayer) (+ (Variables|/Game/Character/Character_Build/BP_CharacterBuild.BP_CharacterBuild_C|GetMana (Variables|Default|GetPlayer)) 1.0))
      (Variables|/Game/Strectching/BP_Platform.BP_Platform_C|SetScale%20Platform _hittenplatform (Math|Vector|MakeVector (- (.x (Variables|/Game/Strectching/BP_Platform.BP_Platform_C|GetScale%20Platform _hittenplatform)) 1.0) (.y (Variables|/Game/Strectching/BP_Platform.BP_Platform_C|GetScale%20Platform _hittenplatform)) (- (.z (Variables|/Game/Strectching/BP_Platform.BP_Platform_C|GetScale%20Platform _hittenplatform)) 1.0))))))