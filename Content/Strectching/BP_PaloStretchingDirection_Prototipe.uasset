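; Prototype stretchable pole actor that detects when the player is close enough and has it in view to begin stretching it.
; It caches the BP_CharacterBuild at BeginPlay, then each Tick shows its text render while the player is within DistanceFromPlayer.
; ProjectWorldToScreen serves as a rough looking-at test.
; When that, proximity and CanPlayerStretchThis all hold, it sets StartStretching, which nothing here resets or consumes.
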(event EventBeginPlay
  (bind _returnvalue (Actor|GetActorOfClass "/Game/Character/Character_Build/BP_CharacterBuild.BP_CharacterBuild_C"))
  (Variables|Default|SetPlayer _returnvalue))

(event EventTick
  (params (DeltaSeconds :type Float%20%28single-precision%29))
  (if (< (Math|Vector|VectorLength (- (Transformation|GetActorLocation (Variables|Default|GetPlayer)) (Transformation|GetActorLocation))) (Variables|Default|GetDistanceFromPlayer))
    (Variables|Default|SetIsPlayerNearToStretchThis? true)
    (Rendering|SetVisibility (Variables|Default|GetTextRender) true false)
    (else
      (Variables|Default|SetIsPlayerNearToStretchThis? false)
      (Rendering|SetVisibility (Variables|Default|GetTextRender) false false)))
  (if (.ReturnValue (Class|GameplayStatics|ProjectWorldtoScreen (Game|GetPlayerController 0) (Transformation|GetActorLocation) false))
    (Variables|Default|SetIsPlayerCameraLookingThis? true)
    (if (and (Variables|Default|GetCanPlayerStretchThis?) (Variables|Default|GetIsPlayerNearToStretchThis?))
      (Variables|Default|SetStartStretching? true))
    (else
      (Variables|Default|SetIsPlayerCameraLookingThis? false))))

(fn ConstructionScript)