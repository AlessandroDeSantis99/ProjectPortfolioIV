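; Stretch-direction actor that acts as crouch cover, hiding the player from Bp_enemyBuild enemies cached at BeginPlay.
; Each Tick, a crouching player overlapping the back or forward invisibility volume clears IsPlayerVisible on all enemies; nothing here restores it.
; Nested enemy loops also toggle each volume's collision, off for an overlapping enemy and query-only otherwise.
; When SpawnDir's X scale drops below a threshold, the actor destroys itself after a short delay.
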(event EventTick
  (params (DeltaSeconds :type Float%20%28single-precision%29))
  (bind _invisibilitycrouch_forward (Variables|Default|GetInvisibilityCrouch_Forward))
  (bind _invisibilitycrouch_back (Variables|Default|GetInvisibilityCrouch_Back))
  (if (< (.x (Transformation|GetWorldScale (Variables|Default|GetSpawnDir))) 0.8)
    (Utilities|FlowControl|Delay 0.2)
    (Utilities|FlowControl|DoOnce false
      (:Completed
        (Actor|DestroyActor)))
    (elif (Collision|IsOverlappingActor (Variables|Default|GetInvisibilityCrouch_Back) (Game|Player|GetPlayerPawn 0) :!class /Script/Engine.PrimitiveComponent)
      (bind _asbp_character_build (Utilities|Casting|CastToBP_CharacterBuild (Game|Player|GetPlayerPawn 0))
        (:then
          (if (Variables|/Game/Character/Character_Build/BP_CharacterBuild.BP_CharacterBuild_C|GetIsCrouching? _asbp_character_build)
            (for _array_element (Variables|Default|GetEnemies)
              (Variables|/Game/Character/Character_Build/Guards/Bp_enemyBuild.Bp_enemyBuild_C|SetIsPlayerVisible? _array_element false)
              (for _array_element_2 (Variables|Default|GetEnemies)
                (if (Collision|IsOverlappingActor (Variables|Default|GetInvisibilityCrouch_Back) _array_element_2 :!class /Script/Engine.PrimitiveComponent)
                  (Collision|SetCollisionEnabled _invisibilitycrouch_back "NoCollision")
                  (else
                    (Collision|SetCollisionEnabled _invisibilitycrouch_back "QueryOnly")))
                (if (Collision|IsOverlappingActor (Variables|Default|GetInvisibilityCrouch_Forward) (Game|Player|GetPlayerPawn 0) :!class /Script/Engine.PrimitiveComponent)
                  (bind _asbp_character_build_2 (Utilities|Casting|CastToBP_CharacterBuild (Game|Player|GetPlayerPawn 0))
                    (:then
                      (if (Variables|/Game/Character/Character_Build/BP_CharacterBuild.BP_CharacterBuild_C|GetIsCrouching? _asbp_character_build_2)
                        (for _array_element_3 (Variables|Default|GetEnemies)
                          (Variables|/Game/Character/Character_Build/Guards/Bp_enemyBuild.Bp_enemyBuild_C|SetIsPlayerVisible? _array_element_3 false)
                          (for _array_element_4 (Variables|Default|GetEnemies)
                            (if (Collision|IsOverlappingActor (Variables|Default|GetInvisibilityCrouch_Forward) _array_element_4 :!class /Script/Engine.PrimitiveComponent)
                              (Collision|SetCollisionEnabled _invisibilitycrouch_forward "NoCollision")
                              (else
                                (Collision|SetCollisionEnabled _invisibilitycrouch_forward "QueryOnly")))))
                        (else
                          (for _array_element_5 (Variables|Default|GetEnemies) :!label _label
                            (if (Collision|IsOverlappingActor (Variables|Default|GetInvisibilityCrouch_Forward) _array_element_5 :!class /Script/Engine.PrimitiveComponent)
                              (Collision|SetCollisionEnabled _invisibilitycrouch_forward "NoCollision")
                              (else
                                (Collision|SetCollisionEnabled _invisibilitycrouch_forward "QueryOnly")))))))
                    (:CastFailed
                      (goto _label)))
                  (else
                    (goto _label)))))
            (else
              (for _array_element_6 (Variables|Default|GetEnemies) :!label _label_2
                (if (Collision|IsOverlappingActor (Variables|Default|GetInvisibilityCrouch_Back) _array_element_6 :!class /Script/Engine.PrimitiveComponent)
                  (Collision|SetCollisionEnabled _invisibilitycrouch_back "NoCollision")
                  (else
                    (Collision|SetCollisionEnabled _invisibilitycrouch_back "QueryOnly")))
                (if (Collision|IsOverlappingActor (Variables|Default|GetInvisibilityCrouch_Forward) (Game|Player|GetPlayerPawn 0) :!class /Script/Engine.PrimitiveComponent)
                  (bind _asbp_character_build_3 (Utilities|Casting|CastToBP_CharacterBuild (Game|Player|GetPlayerPawn 0))
                    (:then
                      (if (Variables|/Game/Character/Character_Build/BP_CharacterBuild.BP_CharacterBuild_C|GetIsCrouching? _asbp_character_build_3)
                        (for _array_element_7 (Variables|Default|GetEnemies)
                          (Variables|/Game/Character/Character_Build/Guards/Bp_enemyBuild.Bp_enemyBuild_C|SetIsPlayerVisible? _array_element_7 false)
                          (for _array_element_8 (Variables|Default|GetEnemies)
                            (if (Collision|IsOverlappingActor (Variables|Default|GetInvisibilityCrouch_Forward) _array_element_8 :!class /Script/Engine.PrimitiveComponent)
                              (Collision|SetCollisionEnabled _invisibilitycrouch_forward "NoCollision")
                              (else
                                (Collision|SetCollisionEnabled _invisibilitycrouch_forward "QueryOnly")))))
                        (else
                          (for _array_element_9 (Variables|Default|GetEnemies) :!label _label_3
                            (if (Collision|IsOverlappingActor (Variables|Default|GetInvisibilityCrouch_Forward) _array_element_9 :!class /Script/Engine.PrimitiveComponent)
                              (Collision|SetCollisionEnabled _invisibilitycrouch_forward "NoCollision")
                              (else
                                (Collision|SetCollisionEnabled _invisibilitycrouch_forward "QueryOnly")))))))
                    (:CastFailed
                      (goto _label_3)))
                  (else
                    (goto _label_3)))))))
        (:CastFailed
          (goto _label_2)))
      (else
        (goto _label_2)))))

(event EventBeginPlay
  (bind _outactors (Actor|GetAllActorsOfClass "/Game/Character/Character_Build/Guards/Bp_enemyBuild.Bp_enemyBuild_C"))
  (Variables|Default|SetEnemies _outactors))

(fn ConstructionScript)