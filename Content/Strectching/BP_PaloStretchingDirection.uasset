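; BP_PaloStretchingDirection is a pole actor that decides when the player can stretch, lighting up when they are near.
; On Tick, proximity, on-screen projection, the player not looking at a platform and a collider overlap flag gate StartStretching.
; When active, it moves the StretchingManager's array matching the player's DirToStretch into its own.
; At BeginPlay, it disables collision on cubes for non-previewable directions.
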(event OnComponentBeginOverlap(Cube1_Collider)
  (params (OverlappedComponent :type Primitive%20Component%20Object%20Reference) (OtherActor :type Actor%20Object%20Reference) (OtherComp :type Primitive%20Component%20Object%20Reference) (OtherBodyIndex :type Integer) (bFromSweep :type Boolean) (SweepResult :type Hit%20Result%20Structure%20%28by%20ref%29))
  ;[0.5844 0.1163 0.154] Collision Check
  (Utilities|Casting|CastToBP_CharacterBuild OtherActor)
  (Variables|Default|SetCanPlayerStretchThis? false))

(event OnComponentEndOverlap(Cube1_Collider)
  (params (OverlappedComponent :type Primitive%20Component%20Object%20Reference) (OtherActor :type Actor%20Object%20Reference) (OtherComp :type Primitive%20Component%20Object%20Reference) (OtherBodyIndex :type Integer))
  ;[0.5844 0.1163 0.154] Collision Check
  (Utilities|Casting|CastToBP_CharacterBuild OtherActor)
  (Variables|Default|SetCanPlayerStretchThis? true))

(event EventBeginPlay
  (bind _returnvalue (Actor|GetActorOfClass "/Game/Character/Character_Build/BP_CharacterBuild.BP_CharacterBuild_C"))
  (Variables|Default|SetPlayer _returnvalue)
  (bind _returnvalue_2 (Actor|GetActorOfClass "/Game/Strectching/BP_StretchingManager.BP_StretchingManager_C"))
  (Variables|Default|SetStretching%20Manager _returnvalue_2)
  (bind _outactors (Actor|GetAllActorsOfClass "BP_PaloStretchingDirection_C"))
  (Variables|Default|SetStretching%20Dir _outactors)
  (|Collision))

(event EventTick
  (params (DeltaSeconds :type Float%20%28single-precision%29))
  (bind _stretching_manager (Variables|Default|GetStretching%20Manager))
  (bind _player (Variables|Default|GetPlayer))
  (bind _player_2 (Variables|Default|GetPlayer))
  (bind _palo_mesh (Variables|Default|GetPalo_Mesh))
  (bind _dirtostretch (Variables|/Game/Character/Character_Build/BP_CharacterBuild.BP_CharacterBuild_C|GetDirToStretch _player_2))
  (if (< (Math|Vector|VectorLength (- (Transformation|GetActorLocation (Variables|Default|GetPlayer)) (Transformation|GetActorLocation))) (Variables|Default|GetDistanceFromPlayer))
    (Components|Activation|Activate (Variables|Default|GetP_Wraith_Drone_Targeting) false)
    (Rendering|Material|SetMaterial _palo_mesh 0 "/Game/SoulCity/Environment/Materials/Building/M_Soul_Glowstick_acceso.M_Soul_Glowstick_acceso")
    (Components|Activation|Activate (Variables|/Game/Character/Character_Build/BP_CharacterBuild.BP_CharacterBuild_C|GetNiagara3 (Variables|Default|GetPlayer)) false)
    (Variables|Default|SetIsPlayerNearToStretchThis? true)
    (if (.ReturnValue (Class|GameplayStatics|ProjectWorldtoScreen (Game|GetPlayerController 0) (Transformation|GetActorLocation) false))
      (Variables|Default|SetIsPlayerCameraLookingThis? true)
      (bind _asbp_character_build (Utilities|Casting|CastToBP_CharacterBuild (Game|Player|GetPlayerPawn 0)))
      (if (Variables|/Game/Character/Character_Build/BP_CharacterBuild.BP_CharacterBuild_C|GetIsLookingAtPlatform? _asbp_character_build)
        (Variables|Default|SetIsPlayerNearToStretchThis? false)
        (for _array_element (Variables|Default|GetStretching%20Dir)
          (Rendering|SetVisibility (Variables|BP_PaloStretchingDirection_C|GetCube1_Collider _array_element) false false))
        (else
          (Variables|Default|SetIsPlayerNearToStretchThis? true)
          (if (and (Variables|Default|GetCanPlayerStretchThis?) (Variables|Default|GetIsPlayerNearToStretchThis?))
            (Variables|Default|SetStartStretching? true)
            (if (== (Variables|/Game/Character/Character_Build/BP_CharacterBuild.BP_CharacterBuild_C|GetPalo%20Steatch%20Dir_1 _player) _dirtostretch)
              (for _array_element_2 (Variables|/Game/Strectching/BP_StretchingManager.BP_StretchingManager_C|GetDirStretch_0 _stretching_manager)
                (Utilities|Array|Add (Variables|Default|GetDirsStretch_0) _array_element_2)
                (Variables|/Game/Strectching/BP_StretchingManager.BP_StretchingManager_C|SetDirStretch_0 _stretching_manager (Variables|Default|GetDirsStretch_Null)))
              (elif (== (Variables|/Game/Character/Character_Build/BP_CharacterBuild.BP_CharacterBuild_C|GetPalo%20Steatch%20Dir_2 _player) _dirtostretch)
                (for _array_element_3 (Variables|/Game/Strectching/BP_StretchingManager.BP_StretchingManager_C|GetDirStretch_1 _stretching_manager)
                  (Utilities|Array|Add (Variables|Default|GetDirsStretch_1) _array_element_3)
                  (Variables|/Game/Strectching/BP_StretchingManager.BP_StretchingManager_C|SetDirStretch_1 _stretching_manager (Variables|Default|GetDirsStretch_Null)))
                (elif (== (Variables|/Game/Character/Character_Build/BP_CharacterBuild.BP_CharacterBuild_C|GetPalo%20Steatch%20Dir_3 _player) _dirtostretch)
                  (for _array_element_4 (Variables|/Game/Strectching/BP_StretchingManager.BP_StretchingManager_C|GetDirStretch_2 _stretching_manager)
                    (Utilities|Array|Add (Variables|Default|GetDirsStretch_2) _array_element_4)
                    (Variables|/Game/Strectching/BP_StretchingManager.BP_StretchingManager_C|SetDirStretch_2 _stretching_manager (Variables|Default|GetDirsStretch_Null)))
                  (elif (== (Variables|/Game/Character/Character_Build/BP_CharacterBuild.BP_CharacterBuild_C|GetPalo%20Steatch%20Dir_4%20 _player) _dirtostretch)
                    (for _array_element_5 (Variables|/Game/Strectching/BP_StretchingManager.BP_StretchingManager_C|GetDirStretch_3 _stretching_manager)
                      (Utilities|Array|Add (Variables|Default|GetDirsStretch_3) _array_element_5)
                      (Variables|/Game/Strectching/BP_StretchingManager.BP_StretchingManager_C|SetDirStretch_3 _stretching_manager (Variables|Default|GetDirsStretch_Null)))))))
            (else
              (Variables|Default|SetStartStretching? false)))))
      (else
        (Variables|Default|SetIsPlayerCameraLookingThis? false)
        (Variables|Default|SetStartStretching? false)))
    (else
      (Components|Activation|Deactivate (Variables|Default|GetP_Wraith_Drone_Targeting))
      (Rendering|Material|SetMaterial _palo_mesh 0 "/Game/SoulCity/Environment/Materials/Props/M_Soul_Glowstick_RK.M_Soul_Glowstick_RK")
      (Components|Activation|Deactivate (Variables|/Game/Character/Character_Build/BP_CharacterBuild.BP_CharacterBuild_C|GetNiagara3 (Variables|Default|GetPlayer)))
      (Variables|Default|SetIsPlayerNearToStretchThis? false))))

(fn ConstructionScript)